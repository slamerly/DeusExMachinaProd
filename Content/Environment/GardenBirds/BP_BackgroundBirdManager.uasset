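; Manager actor that sends pooled background birds flying along its forward axis as garden ambience.
; A timer driven by the BirdTimings list launches birds from a pre-spawned pool, which grows when all are in use.
; Tick moves each active bird forward with a sine vertical bob, then hides and frees it at MaximumLength.
; The construction script draws a debug line showing the flight path.
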(event Custom|SpawnNextBird
  (CallFunction|PrepareNextTimer)
  (CallFunction|PrepareNextBird))

(event EventBeginPlay
  (Variables|Default|SetCachedForward (Transformation|GetActorForwardVector))
  ;[0.5104 1 1] Prepare the pool with 3 birds
  (CallFunction|SpawnFreshBird)
  (CallFunction|SpawnFreshBird)
  (CallFunction|SpawnFreshBird)
  (CallFunction|SpawnFreshBird)
  ;[0.9083 0.4099 1] Start the cycle
  (CallFunction|SpawnNextBird))

(event EventTick
  (params (DeltaSeconds :type Float%20%28single-precision%29))
  (CallFunction|MoveEachBird DeltaSeconds))

(fn ConstructionScript
  (bind _returnvalue (Transformation|GetActorLocation))
  (Rendering|Debug|FlushPersistentDebugLines)
  (Rendering|Debug|DrawDebugLine _returnvalue (+ _returnvalue (* (Transformation|GetActorForwardVector) (Variables|Default|GetMaximum%20Length))) "(R=0.000000,G=0.416667,B=0.027380,A=1.000000)" 1e+01 3.0))

(fn PrepareNextTimer
  (bind _nextelement (CallFunction|PickNextElement (Variables|Default|GetBird%20Timings)))
  (Utilities|Time|SetTimerbyEvent (EventDispatchers|CreateEvent :!event Custom|SpawnNextBird) (* (Math|Conversions|ToFloat(Integer) _nextelement) 0.5)))

(fn SpawnFreshBird
  (bind _returnvalue (Game|SpawnActorfromClass "/Game/Environment/GardenBirds/BP_BackgroundBird.BP_BackgroundBird_C" (Math|Transform|MakeTransform "0.000000,0.000000,-5000.000000" (Transformation|GetActorRotation) "1.000000,1.000000,1.000000") "Undefined" "MultiplyWithRoot" 0 0))
  (Rendering|SetActorHiddenInGame _returnvalue true)
  (Utilities|Array|Add (Variables|Default|GetBird%20Pool) _returnvalue)
  (Variables|/Game/Environment/GardenBirds/BP_BackgroundBird.BP_BackgroundBird_C|SetbIsAvailable _returnvalue true)
  (return _returnvalue))

(fn PrepareNextBird
  (LocalVariables|SetisBirdValid false)
  ;[0.5521 0.4062 1] Get the first available bird from the pool
  (bind _array_element (Utilities|Array|ForEachLoopwithBreak (Variables|Default|GetBird%20Pool) :!label _label)
    (:LoopBody
      (if (Variables|/Game/Environment/GardenBirds/BP_BackgroundBird.BP_BackgroundBird_C|GetbIsAvailable _array_element)
        (LocalVariables|SetisBirdValid true)
        (goto _label Break)))
    (:Completed
      (if (LocalVariables|GetisBirdValid)
        ;[0.2552 0.08906 0.1616] Get the valid Bird from the cached data
        (LocalVariables|SetBirdToPrepare _array_element)
        (else
          (Development|PrintString "ALL POOLED BIRDS ARE USED, SPAWNING NEW ONE" true true "(R=1.000000,G=0.000000,B=0.000000,A=1.000000)")
          (bind _returnvalue (CallFunction|SpawnFreshBird))
          (LocalVariables|SetBirdToPrepare _returnvalue)))
      ;[0.3 0.3762 1] Set all starting values
      (Variables|/Game/Environment/GardenBirds/BP_BackgroundBird.BP_BackgroundBird_C|SetCurrentTime (LocalVariables|GetBirdToPrepare) 0.0)
      (Variables|/Game/Environment/GardenBirds/BP_BackgroundBird.BP_BackgroundBird_C|SetbIsAvailable (LocalVariables|GetBirdToPrepare) false)
      (Rendering|SetActorHiddenInGame (LocalVariables|GetBirdToPrepare) false)
      (Transformation|SetActorLocation (LocalVariables|GetBirdToPrepare) (Transformation|GetActorLocation) false false))))

(fn MoveEachBird
  (params (Delta%20Time :type Float%20%28double-precision%29))
  (for _array_element (Variables|Default|GetBird%20Pool)
    (if (not (Variables|/Game/Environment/GardenBirds/BP_BackgroundBird.BP_BackgroundBird_C|GetbIsAvailable _array_element))
      (LocalVariables|SetCurrentBird _array_element)
      ;[0.3284 1 0.7338] Increase Bird's Internal Current Time
      (CallFunction|IncreaseValueFloat (Variables|/Game/Environment/GardenBirds/BP_BackgroundBird.BP_BackgroundBird_C|GetCurrentTime (LocalVariables|GetCurrentBird)) Delta%20Time)
      ;[1 0.2083 0.2182] Horizontal Movement
      (LocalVariables|SetCurrent%20Horizontal%20Movement (* (Variables|Default|GetBirdHorizontalSpeed) (Variables|/Game/Environment/GardenBirds/BP_BackgroundBird.BP_BackgroundBird_C|GetCurrentTime (LocalVariables|GetCurrentBird))))
      ;[1 0.963 0.3991] Check if the Bird has attained the end of the road
      (if (>= (LocalVariables|GetCurrent%20Horizontal%20Movement) (Variables|Default|GetMaximum%20Length))
        (CallFunction|FreeBird (LocalVariables|GetCurrentBird))
        (else
          (Transformation|SetActorLocation (LocalVariables|GetCurrentBird) (+ (Transformation|GetActorLocation) (* (Variables|Default|GetCachedForward) (LocalVariables|GetCurrent%20Horizontal%20Movement)) (Math|Vector|MakeVector 0.0 0.0 (CallFunction|CustomSineRadians (Variables|/Game/Environment/GardenBirds/BP_BackgroundBird.BP_BackgroundBird_C|GetCurrentTime (LocalVariables|GetCurrentBird)) (Variables|Default|GetBird%20Vertical%20Frequency) (Variables|Default|GetBird%20Vertical%20Amplitude)))) false false))))))

(fn FreeBird
  (params (BirdToRelease :type BP%20Background%20Bird%20Object%20Reference))
  (Variables|/Game/Environment/GardenBirds/BP_BackgroundBird.BP_BackgroundBird_C|SetbIsAvailable BirdToRelease true)
  (Transformation|SetActorLocation BirdToRelease "0.000000,0.000000,-5000.000000" false false)
  (Rendering|SetActorHiddenInGame BirdToRelease true))