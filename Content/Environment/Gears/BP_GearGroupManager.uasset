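; Manager actor that drives every BP_SynchronizedGear in indexed groups, turning them notch by notch with pauses between steps.
; On BeginPlay it buckets gears by group index, seeds per-group state maps and prints errors for mis-sized timing maps.
; Tick alternates each active group between wait and move timers, rotating gears by per-type notch angle over group time, signed by direction, so no gear type is the reference.
; Groups have start/stop functions.
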(event EventBeginPlay
  (Initialization|ReferenceAllGears)
  (Initialization|InitializeMaps))

(event EventTick
  (params (DeltaSeconds :type Float%20%28single-precision%29))
  ;[0.03155 0.1354 0.02468] Delta Time (or Delta Seconds) is gonna be used A LOT each frame.
  ; So we cache it!
  (Variables|Default|SetCached%20Delta%20Time DeltaSeconds)
  ;[0.0948 0.1302 0.05421] Start the Loop!!
  (for _array_element (Variables|Initialization|GetAll%20Gear%20Group%20Indexes)
    (Variables|Default|SetCurrent%20Group%20Index _array_element)
    ;[0.03523 0.1354 0.044] Before doing anything, should this Gear Group even move?
    (if (.Value (Utilities|Map|Find (Variables|Movement|GetShould%20This%20Group%20Move) (Variables|Default|GetCurrent%20Group%20Index)))
      ;[0.07028 0.1979 0.1317] Is this group in a Waiting phase or a Moving phase?
      (if (.Value (Utilities|Map|Find (Variables|Movement|GetIs%20This%20Group%20Currently%20Moving) (Variables|Default|GetCurrent%20Group%20Index)))
        (Movement|MoveGroup)
        (else
          (Waiting|IncreaseGroupWaitTimer))))))

(fn ConstructionScript)

(fn StartMovingGearGroup
  (params (Gear%20Group%20To%20Move :type Integer))
  (if (.ReturnValue (Utilities|Map|Find (Variables|Movement|GetShould%20This%20Group%20Move) Gear%20Group%20To%20Move))
    (Utilities|Map|Add (Variables|Movement|GetShould%20This%20Group%20Move) Gear%20Group%20To%20Move true)))

(fn StopMovingGearGroup
  (params (Gear%20Group%20To%20Move :type Integer))
  (if (.ReturnValue (Utilities|Map|Find (Variables|Movement|GetShould%20This%20Group%20Move) Gear%20Group%20To%20Move))
    (Utilities|Map|Add (Variables|Movement|GetShould%20This%20Group%20Move) Gear%20Group%20To%20Move false)))

(fn ReferenceAllGears
  ;[0.125 0.03776 0.03776] Messy Spaghetti but this is ok
  (bind _outactors (Actor|GetAllActorsOfClass "/Game/Environment/Gears/BP_SynchronizedGear.BP_SynchronizedGear_C"))
  (for _array_element _outactors
    (bind _output_get (LocalVariables|Set_CurrentArray (.actors (.Value (Utilities|Map|Find (Variables|Default|GetAll%20Gears) (Variables|/Game/Environment/Gears/BP_SynchronizedGear.BP_SynchronizedGear_C|GetGear%20Group%20Index _array_element))))))
    (Utilities|Array|Add _output_get _array_element)
    (Utilities|Map|Add (Variables|Default|GetAll%20Gears) (Variables|/Game/Environment/Gears/BP_SynchronizedGear.BP_SynchronizedGear_C|GetGear%20Group%20Index _array_element) (Utilities|Struct|MakeSTR_ActorArray _output_get)))
  (bind _keys (Utilities|Map|Keys (Variables|Default|GetAll%20Gears)))
  (Variables|Initialization|SetAll%20Gear%20Group%20Indexes _keys))

(fn InitializeMaps
  (bind _wait_time_per_group (Variables|Setup|GetWait%20Time%20Per%20Group))
  (bind _all_gear_group_indexes (Variables|Initialization|GetAll%20Gear%20Group%20Indexes))
  (bind _all_gear_group_indexes_2 (Variables|Initialization|GetAll%20Gear%20Group%20Indexes))
  (bind _rotation_time_per_group__per_notch_ (Variables|Setup|GetRotation%20Time%20per%20Group%20%28per%20notch%29))
  (bind _returnvalue (Utilities|Array|Length _all_gear_group_indexes_2))
  (bind _returnvalue_2 (Utilities|Array|Length _all_gear_group_indexes))
  (bind _returnvalue_3 (Utilities|Map|Length _rotation_time_per_group__per_notch_))
  (bind _returnvalue_4 (Utilities|Map|Length _wait_time_per_group))
  (for _array_element (Variables|Initialization|GetAll%20Gear%20Group%20Indexes)
    (LocalVariables|SetCurrent%20Initializing%20Group%20Index _array_element)
    ;[1 0.194 0.1442] Should Move?
    (Utilities|Map|Add (Variables|Movement|GetShould%20This%20Group%20Move) (LocalVariables|GetCurrent%20Initializing%20Group%20Index) (.Value (Utilities|Map|Find (Variables|Setup|GetStart%20Moving%20On%20Begin%20Play) (LocalVariables|GetCurrent%20Initializing%20Group%20Index))))
    ;[0.2336 1 0.2476] Starting Rotation
    (Utilities|Map|Add (Variables|Movement|GetGears%20Current%20Timer) (LocalVariables|GetCurrent%20Initializing%20Group%20Index) 0.0)
    ;[1 0.2083 0.639] Is this group currently moving?
    (Utilities|Map|Add (Variables|Movement|GetIs%20This%20Group%20Currently%20Moving) (LocalVariables|GetCurrent%20Initializing%20Group%20Index) false))
  ;[1 0 0] DATA  VALIDATION  ERROR  DEBUG
  (if (!= _returnvalue_2 _returnvalue_4)
    (Development|PrintText (Utilities|Text|FormatText "BP_GearGroupManager: 
\"Wait Time Per Group\" map isn't the right length! 
Expecting a length of {ex} but current length is {cu}" _returnvalue_2 _returnvalue_4) true true "(R=1.000000,G=0.000000,B=0.000000,A=1.000000)" 5e+01))
  (if (!= _returnvalue _returnvalue_3)
    (Development|PrintText (Utilities|Text|FormatText "BP_GearGroupManager: 
\"Rotation Time per Group (per notch)\" map isn't the right length! 
Expecting a length of {ex} but current length is {cu}" _returnvalue _returnvalue_3) true true "(R=1.000000,G=0.000000,B=0.000000,A=1.000000)" 5e+01)))

(fn IncreaseGroupWaitTimer
  ;[1 0.4518 0.8066] Increase Timer
  (bind _output_get (LocalVariables|SetFinal%20Group%20Timer (+ (.Value (Utilities|Map|Find (Variables|Movement|GetGears%20Current%20Timer) (Variables|Default|GetCurrent%20Group%20Index))) (Variables|Default|GetCached%20Delta%20Time))))
  ;[0.6151 0.492 1] Have we waited enough to start moving next frame?
  (if (>= _output_get (.Value (Utilities|Map|Find (Variables|Setup|GetWait%20Time%20Per%20Group) (Variables|Default|GetCurrent%20Group%20Index))))
    ;[0.1562 0.1234 0.07356] Reset timer and Start Moving! (next frame)
    (Utilities|Map|Add (Variables|Movement|GetGears%20Current%20Timer) (Variables|Default|GetCurrent%20Group%20Index) 0.0)
    (Utilities|Map|Add (Variables|Movement|GetIs%20This%20Group%20Currently%20Moving) (Variables|Default|GetCurrent%20Group%20Index) true)
    (else
      ;[0.1146 0.08057 0.08057] Just increment the timer
      (Utilities|Map|Add (Variables|Movement|GetGears%20Current%20Timer) (Variables|Default|GetCurrent%20Group%20Index) (LocalVariables|GetFinal%20Group%20Timer)))))

(fn MoveGroup
  (LocalVariables|SetRotation%20Time%20For%20This%20Group (.Value (Utilities|Map|Find (Variables|Setup|GetRotation%20Time%20per%20Group%20%28per%20notch%29) (Variables|Default|GetCurrent%20Group%20Index))))
  (bind _output_get (LocalVariables|SetGroup%20Pre-Rotation (/ (Variables|Default|GetCached%20Delta%20Time) (LocalVariables|GetRotation%20Time%20For%20This%20Group))))
  (LocalVariables|SetNegative%20Pre-Rotation (* _output_get -1.0))
  (bind _output_get_2 (LocalVariables|SetAll%20Gears%20To%20Rotate (.Value (Utilities|Map|Find (Variables|Default|GetAll%20Gears) (Variables|Default|GetCurrent%20Group%20Index)))))
  (for _array_element (.actors _output_get_2)
    ;[0.06982 0.1719 0.1101] Rotate each gear by the right amount
    ; Gear-dependent speed * 1 or -1 for the direction * Delta Time
    ; Everything / by the time this group must take to do a one-notch rotation
    ;
    ; This gives us a way to rotate everything without setting a gear type as the "basis"
    ;
    ; Separate to avoid multiplying by 1 or -1 all the time and avoid as much math as possible
    (bind _gear_type (Class|BPIGearInterface|GetGearType(Message) _array_element))
    (bind _is_clockwise (Class|BPIGearInterface|GetIsRotatingClockwise(Message) _array_element))
    (if _is_clockwise
      (Transformation|AddActorLocalRotation _array_element (Math|Rotator|MakeRotator 0.0 0.0 (* (LocalVariables|GetGroup%20Pre-Rotation) (.Value (Utilities|Map|Find (Variables|Movement|GetRotation%20To%20Do%20One%20Notch) _gear_type)))) false true)
      (else
        (Transformation|AddActorLocalRotation _array_element (Math|Rotator|MakeRotator 0.0 0.0 (* (LocalVariables|GetNegative%20Pre-Rotation) (.Value (Utilities|Map|Find (Variables|Movement|GetRotation%20To%20Do%20One%20Notch) _gear_type)))) false true))))
  ;[1 0.4518 0.8066] Increase Timer
  (LocalVariables|SetFinal%20Group%20Timer (+ (.Value (Utilities|Map|Find (Variables|Movement|GetGears%20Current%20Timer) (Variables|Default|GetCurrent%20Group%20Index))) (Variables|Default|GetCached%20Delta%20Time)))
  ;[0.6151 0.492 1] Have we waited enough to stop moving next frame?
  (if (>= (LocalVariables|GetFinal%20Group%20Timer) (.Value (Utilities|Map|Find (Variables|Setup|GetRotation%20Time%20per%20Group%20%28per%20notch%29) (Variables|Default|GetCurrent%20Group%20Index))))
    ;[0.1562 0.1234 0.07356] Reset timer and Stop Moving! (next frame)
    (Utilities|Map|Add (Variables|Movement|GetGears%20Current%20Timer) (Variables|Default|GetCurrent%20Group%20Index) 0.0)
    (Utilities|Map|Add (Variables|Movement|GetIs%20This%20Group%20Currently%20Moving) (Variables|Default|GetCurrent%20Group%20Index) false)
    (else
      ;[0.1146 0.08057 0.08057] Just increment the timer
      (Utilities|Map|Add (Variables|Movement|GetGears%20Current%20Timer) (Variables|Default|GetCurrent%20Group%20Index) (LocalVariables|GetFinal%20Group%20Timer)))))