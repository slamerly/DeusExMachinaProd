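; Synchronized gear actor that takes its mesh from GearType and exposes its type and rotation direction through getters; no rotation logic lives here.
; The Construction Script applies a dynamic trigger-box material colored by gear group, repurposing its isOneTimeUse parameter to mark counter-clockwise gears, and warns about X/Y scaling.
; BeginPlay swaps that material for the gear type's own, so the color coding serves as an editor preview.
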(event EventBeginPlay
  (bind _material (CallFunction|GetGearMaterial (Variables|Setup|GetGear%20Type)))
  (Rendering|Material|SetMaterial (Variables|Default|GetStaticMesh) 0 _material))

(fn ConstructionScript
  (bind _returnvalue (Transformation|GetActorScale3D))
  (bind _static_mesh (CallFunction|GetGearMesh (Variables|Setup|GetGear%20Type)))
  (Components|StaticMesh|SetStaticMesh (Variables|Default|GetStaticMesh) _static_mesh)
  (Variables|Default|GetMaterialInstance
    (:then
      _)
    (:else
      (bind _returnvalue_2 (Rendering|Material|CreateDynamicMaterialInstance (Variables|Default|GetStaticMesh) 0 "/UpgradedTriggerBoxes/Materials/MI_Trigger_BoxMaterial.MI_Trigger_BoxMaterial" "None" :!class /Script/Engine.PrimitiveComponent))
      (bind _output_get (Variables|Default|SetMaterialInstance _returnvalue_2))
      (Rendering|Material|SetScalarParameterValue _output_get "Opacity" 1.0 :!class /Script/Engine.MaterialInstanceDynamic)))
  (Rendering|Material|SetVectorParameterValue (Variables|Default|GetMaterialInstance) "BaseColor" (CallFunction|GetPlayerColorfromIndex (Variables|Setup|GetGear%20Group%20Index)) :!class /Script/Engine.MaterialInstanceDynamic)
  (Rendering|Material|SetScalarParameterValue (Variables|Default|GetMaterialInstance) "isOneTimeUse" (Math|Conversions|ToFloat(Boolean) (not (Variables|Setup|GetRotates%20Clockwise?))) :!class /Script/Engine.MaterialInstanceDynamic)
  ;[0.6147 0.4092 1] Allow for scaling on Z but not the others
  (if (Class|KismetMathLibrary|NotEqualExactlyVector2DVector2D (Math|Vector2D|MakeVector2D (.x _returnvalue) (.y _returnvalue)) "(X=1.000000,Y=1.000000)")
    (Development|PrintString "Be careful to only scale Gears if you absolutely need to!!! 
To have bigger gears relative to other gears, just change the Gear Type, speeds are then automatically adjusted!!!!" true true "(R=1.000000,G=0.000000,B=0.000000,A=1.000000)" 5e+01 "GearNoScaling")))

(fn GetGearType
  (return (Variables|Setup|GetGear%20Type)))

(fn GetIsRotatingClockwise
  (return (Variables|Setup|GetRotates%20Clockwise?)))