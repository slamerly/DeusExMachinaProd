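; Player character Blueprint that sets ground movement speed for walking and trotting.
; On BeginPlay it calls the parent and sets the CharacterMovement max walk speed to the walking value from PlayerSpeeds.
; The Switch Movement Speed function toggles that max speed between the trot and walking values based on a boolean.
; Tick only forwards to the parent, and the construction script is empty.
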(event EventTick
  (params (DeltaSeconds :type Float%20%28single-precision%29))
  ;[0 1 0] EVENT TICK
  (|CallParentFunction DeltaSeconds))

(event EventBeginPlay
  ;[1 0 0] BeginPlay
  (|CallParentFunction)
  (Variables|/Script/Engine.CharacterMovementComponent|SetMaxWalkSpeed (Variables|Character|GetCharacterMovement) (Variables|/Game/Datas/Player/PDA_PlayerSpeeds.PDA_PlayerSpeeds_C|GetWalking%20Speed (Variables|Movement|GetPlayer%20Speeds))))

(fn ConstructionScript)

(fn SwitchMovementSpeed
  (params (Switch%20To%20Trot? :type Boolean))
  (if Switch%20To%20Trot?
    (Variables|/Script/Engine.CharacterMovementComponent|SetMaxWalkSpeed (Variables|Character|GetCharacterMovement) (Variables|/Game/Datas/Player/PDA_PlayerSpeeds.PDA_PlayerSpeeds_C|GetTrot%20Speed (Variables|Movement|GetPlayer%20Speeds)))
    (else
      (Variables|/Script/Engine.CharacterMovementComponent|SetMaxWalkSpeed (Variables|Character|GetCharacterMovement) (Variables|/Game/Datas/Player/PDA_PlayerSpeeds.PDA_PlayerSpeeds_C|GetWalking%20Speed (Variables|Movement|GetPlayer%20Speeds))))))