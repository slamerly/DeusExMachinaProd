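; BP_DialogueBox is a world-placed dialogue box actor that shows narration lines through a WBP_InGameDialogue widget component.
; It forwards display, force-complete and hide requests to that widget, passing itself as owner along with speaker, reading speed and auto-skip delay.
; On completion it sets CurrentDialogueIsFinished on the stored NarrationManager.
; In the editor, a text render shows the box index in its player color and is destroyed at BeginPlay.
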(event Custom|Receive%20Dialogue
  (params (Dialogue%20to%20Show :type Text) (Reading%20Speed :type Float%20%28double-precision%29) (NarrationManager :type BP%20Narration%20Manager%20Object%20Reference) (Automatic%20Skip%20After%20%28Seconds%29 :type Float%20%28double-precision%29) (Dialogue%20Speaker :type EPossibleDialogueSpeakers%20Enum :default "NewEnumerator1"))
  (Default|ReceiveDialogue (Variables|Default|GetWidget%20Class) Dialogue%20to%20Show Reading%20Speed self Automatic%20Skip%20After%20%28Seconds%29 Dialogue%20Speaker)
  (Variables|Default|SetNarration%20Manager NarrationManager))

(event Custom|Force%20Complete%20Dialogue
  (Default|ForceCompleteDialogue (Variables|Default|GetWidget%20Class)))

(event Custom|Dialogue%20Has%20Completed
  (Variables|/Game/Narration/BP_NarrationManager.BP_NarrationManager_C|SetCurrent%20Dialogue%20is%20Finished (Variables|Default|GetNarration%20Manager) true))

(event Custom|Hide%20Dialogue
  (Default|HideDialogue (Variables|Default|GetWidget%20Class)))

(event EventBeginPlay
  (bind _aswbp_in_game_dialogue (Utilities|Casting|CastToWBP_InGameDialogue (UserInterface|GetWidget (Variables|Default|GetWidget))))
  (Variables|Default|SetWidget%20Class _aswbp_in_game_dialogue)
  (Components|DestroyComponent (Variables|Default|GetTextRender)))

(fn ConstructionScript
  (bind _textrender (Variables|Default|GetTextRender))
  (bind _dialogue_box_index (Variables|Default|GetDialogue%20Box%20Index))
  (Rendering|Components|TextRender|SetText _textrender (Utilities|Text|ToText(Integer) _dialogue_box_index))
  (Rendering|Components|TextRender|SetTextRenderColor _textrender (Math|Conversions|ToColor(LinearColor) (CallFunction|GetPlayerColorfromIndex _dialogue_box_index))))