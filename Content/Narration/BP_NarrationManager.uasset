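; BP_NarrationManager runs the game's narration, chaining dialogues and Level Sequence cinematics through follow-up DataTable rows.
; On BeginPlay it indexes every BP_DialogueBox, then routes each line to its box, which reports back on completion.
; Interact input completes or advances the line unless ignored, while per-line flags switch player input between narration and movement.
; Final lines can stop the cinematic, and finished sequences can launch follow-ups.
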(event Custom|Interact%20Input%20Received
  (if (not (.IgnoreUserInputs? (Utilities|Struct|BreakSTR_DialogueValues (Variables|Dialogue|GetCurrent%20Dialogue))))
    (if (Variables|Dialogue|GetCurrent%20Dialogue%20is%20Finished)
      (Dialogue|GotoNextDialogue true)
      (else
        ;[0.5006 1 0.3229] Dialogue is still running, Complete it!
        (Default|ForceCompleteDialogue (Variables|Dialogue|DialogueBoxes|GetCurrent%20Dialogue%20Box))))))

(event Custom|Current%20Dialogue%20Has%20Complete
  ;[0.1138 0.1427 0.3073] Dialogue is finished! Called from the Dialogue Box directly
  (Variables|Dialogue|SetCurrent%20Dialogue%20is%20Finished true))

(event Custom|Current%20Cinematic%20is%20Finished
  (bind _current_cinematic (Variables|Cinematic|GetCurrent%20Cinematic))
  (bind (_hasfollowupcinematic _followupcinematic) (Utilities|Struct|BreakSTR_CinematicValues _current_cinematic))
  (bind (_datatable _rowname) (Utilities|Struct|BreakDataTableRowHandle _followupcinematic))
  ;[0.2602 0.07283 0.2969] Cinematic is Finished!
  ; Called because this event is Bound directly when starting the Cinematic
  (if _hasfollowupcinematic
    (bind _returnvalue (Utilities|GetDataTableRow _datatable _rowname)
      (:then
        (CallFunction|StartNewCinematic _returnvalue))
      (:RowNotFound
        ;[1 0 0] DEBUG ERROR PRINT
        (Development|PrintText (Utilities|Text|FormatText "Found no Row named {row} 
in the Data Table {data}" _rowname (Utilities|GetDisplayName _datatable)) true true "(R=1.000000,G=0.000000,B=0.000000,A=1.000000)" 5e+01)))))

(event EventBeginPlay
  (bind _asplayer_controller_deus_ex (Utilities|Casting|CastToPlayerControllerDeusEx (Game|GetPlayerController 0)))
  (Variables|Default|SetPlayer%20Controller%20Reference _asplayer_controller_deus_ex)
  (Dialogue|RegisterAllDialogueBoxes))

(fn ConstructionScript)

(fn RegisterAllDialogueBoxes
  (Utilities|Map|Clear (Variables|Dialogue|DialogueBoxes|GetAll%20In%20Game%20Dialogue%20Boxes))
  (bind _outactors (Actor|GetAllActorsOfClass "/Game/Narration/BP_DialogueBox.BP_DialogueBox_C"))
  (for _array_element _outactors
    (Utilities|Map|Add (Variables|Dialogue|DialogueBoxes|GetAll%20In%20Game%20Dialogue%20Boxes) (Variables|/Game/Narration/BP_DialogueBox.BP_DialogueBox_C|GetDialogue%20Box%20Index _array_element) _array_element)))

(fn StartNewDialogue
  (params (Next%20Dialogue :type STR%20Dialogue%20Values%20Structure))
  (Variables|Dialogue|SetCurrent%20Dialogue Next%20Dialogue)
  (if (Utilities|Struct|BreakSTR_DialogueValues (Variables|Dialogue|GetCurrent%20Dialogue))
    _
    (else
      (Class|PlayerControllerInterface|SetPlayerInputMode (Variables|Default|GetPlayer%20Controller%20Reference) "NarrationControl")))
  (Variables|Dialogue|SetCurrent%20Dialogue%20is%20Finished false)
  (bind _output_get (Variables|Dialogue|DialogueBoxes|SetCurrent%20Dialogue%20Box (.Value (Utilities|Map|Find (Variables|Dialogue|DialogueBoxes|GetAll%20In%20Game%20Dialogue%20Boxes) (Utilities|Struct|BreakSTR_DialogueValues (Variables|Dialogue|GetCurrent%20Dialogue))))))
  (Default|ReceiveDialogue _output_get (.DialogueKey (Utilities|Struct|BreakSTR_DialogueValues (Variables|Dialogue|GetCurrent%20Dialogue))) (.ReadSpeed (Utilities|Struct|BreakSTR_DialogueValues (Variables|Dialogue|GetCurrent%20Dialogue))) self (Math|Float|SelectFloat (.SkipAutomaticallyAfterSeconds (Utilities|Struct|BreakSTR_DialogueValues (Variables|Dialogue|GetCurrent%20Dialogue))) 0.0 (or (.IgnoreUserInputs? (Utilities|Struct|BreakSTR_DialogueValues (Variables|Dialogue|GetCurrent%20Dialogue))) (.DontFreezePlayer? (Utilities|Struct|BreakSTR_DialogueValues (Variables|Dialogue|GetCurrent%20Dialogue))))) (.SpeakerName (Utilities|Struct|BreakSTR_DialogueValues (Variables|Dialogue|GetCurrent%20Dialogue)))))

(fn GotoNextDialogue
  (params (Can%20Give%20Back%20Inputs? :type Boolean))
  (bind _current_dialogue (Variables|Dialogue|GetCurrent%20Dialogue))
  (bind (_hasfollowup_ _nextdialogue) (Utilities|Struct|BreakSTR_DialogueValues _current_dialogue))
  (bind (_datatable _rowname) (Utilities|Struct|BreakDataTableRowHandle _nextdialogue))
  ;[1 0.3704 0.906] Go to the next dialogue, if any
  (if _hasfollowup_
    (Default|HideDialogue (Variables|Dialogue|DialogueBoxes|GetCurrent%20Dialogue%20Box))
    (bind _returnvalue (Utilities|GetDataTableRow _datatable _rowname)
      (:then
        ;;[1 0.265 0.1352] If the next dialogue shouldn't freeze the player, give them the inputs back!
        (if (Utilities|Struct|BreakSTR_DialogueValues _returnvalue)
          (Class|PlayerControllerInterface|SetPlayerInputMode (Variables|Default|GetPlayer%20Controller%20Reference) "PlayerMovement"))
        (Dialogue|StartNewDialogue _returnvalue))
      (:RowNotFound
        ;[1 0 0] DEBUG ERROR PRINT
        (Development|PrintText (Utilities|Text|FormatText "Found no Row named {row} 
in the Data Table {data}" _rowname (Utilities|GetDisplayName _datatable)) true true "(R=1.000000,G=0.000000,B=0.000000,A=1.000000)" 5e+01)))
    (else
      ;[1 0.3638 0.3937] No dialogue after this one? Hide the current Dialogue Box!
      (Default|HideDialogue (Variables|Dialogue|DialogueBoxes|GetCurrent%20Dialogue%20Box))
      ;[1 0.4077 0.7458] What's next differs from Cinematic and Gameplay
      (if (Variables|Cinematic|GetIs%20In%20Cinematic)
        ;[0.6678 0.4152 1] In Cinematic, This text can ask to end the cinematic automatically. If so, do and give back everything to the Player.
        ; If it doesn't, it's probably that there's a bit of Cinematic left.
        (if (Utilities|Struct|BreakSTR_DialogueValues (Variables|Dialogue|GetCurrent%20Dialogue))
          (Class|PlayerControllerInterface|SetPlayerInputMode (Variables|Default|GetPlayer%20Controller%20Reference) "PlayerMovement")
          (Sequencer|Player|Stop (Variables|Cinematic|GetLevel%20Sequence%20Player) :!class /Script/MovieScene.MovieSceneSequencePlayer))
        (else
          ;[0.3186 0.3008 1] In gameplay, the Dialogue could have been purely environmental and not freeze player inputs.
          ;
          ; If it did freeze the player though, give the inputs back!
          (if (not (Utilities|Struct|BreakSTR_DialogueValues (Variables|Dialogue|GetCurrent%20Dialogue)))
            (if Can%20Give%20Back%20Inputs?
              (Class|PlayerControllerInterface|SetPlayerInputMode (Variables|Default|GetPlayer%20Controller%20Reference) "PlayerMovement"))))))))

(fn StartNewCinematic
  (params (Cinematic%20to%20Play :type STR%20Cinematic%20Values%20Structure))
  (Variables|Cinematic|SetCurrent%20Cinematic Cinematic%20to%20Play)
  (Variables|Cinematic|SetIs%20In%20Cinematic true)
  (bind _returnvalue (Sequencer|Player|CreateLevelSequencePlayer (.SequencetoPlay (Utilities|Struct|BreakSTR_CinematicValues (Variables|Cinematic|GetCurrent%20Cinematic))) (Utilities|Struct|MakeMovieSceneSequencePlaybackSettings true (Utilities|Struct|MakeMovieSceneSequenceLoopCount (Math|Integer|SelectInt -1 0 (.ShouldLoop? (Utilities|Struct|BreakSTR_CinematicValues (Variables|Cinematic|GetCurrent%20Cinematic))))) 1.0 0.0 false false false false false false "ForceRestoreState")))
  (EventDispatchers|BindEventtoOnFinished _returnvalue (EventDispatchers|CreateEvent :!event Custom|Current%20Cinematic%20is%20Finished))
  (Variables|Cinematic|SetLevel%20Sequence%20Player _returnvalue))