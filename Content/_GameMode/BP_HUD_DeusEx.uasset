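; BP_HUD_DeusEx is a HUD Blueprint that owns the interaction tooltip and a progress widget exposed as the debug menu.
; On BeginPlay it creates both widgets for the first player controller, layers the progress widget above the tooltip, and starts the tooltip hidden.
; Show and hide events forward to the tooltip, with showing taking a screen-fraction position, while GetDebugMenu returns the progress widget.
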(event EventBeginPlay
  (bind _returnvalue (Game|GetPlayerController 0))
  (Utilities|FlowControl|Sequence
    (:then_0
      ;[1 1 1] Tooltip
      (bind _returnvalue_2 (UserInterface|CreateWidget "/Game/UI/Interaction/WBP_InteractionTooltip.WBP_InteractionTooltip_C" _returnvalue))
      (bind _output_get (Variables|Default|SetTooltipWidget _returnvalue_2))
      (UserInterface|Viewport|AddtoViewport _output_get 0)
      (Default|HideTooltip _output_get))
    (:then_1
      (bind _returnvalue_3 (UserInterface|CreateWidget "/Game/Gameplay/ProgressSystem/WBP_Progress.WBP_Progress_C" _returnvalue))
      (bind _output_get_2 (Variables|Default|SetDebugMenu _returnvalue_3))
      (UserInterface|Viewport|AddtoViewport _output_get_2 1))))

(event Collision|EventActorBeginOverlap
  (params (OtherActor :type Actor%20Object%20Reference)))

(event EventTick
  (params (DeltaSeconds :type Float%20%28single-precision%29)))

(event EventShowInteractionTooltip
  (params (TooltipScreenFractionPos :type Vector%202D%20Structure))
  (Default|ShowTooltip (Variables|Default|GetTooltipWidget) TooltipScreenFractionPos))

(event EventHideInteractionTooltip
  (Default|HideTooltip (Variables|Default|GetTooltipWidget)))

(fn ConstructionScript)

(fn GetDebugMenu
  (return (Variables|Default|GetDebugMenu)))