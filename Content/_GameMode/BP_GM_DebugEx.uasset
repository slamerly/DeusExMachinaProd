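; Game mode that gives other objects access to a gameplay-tag-based event dispatcher hub.
; PostLogin spawns and stores BP_EDH_EventDispatcherHub before BeginPlay, so actors can register on their own BeginPlay.
; Its events forward single or multiple bind, unbind and call requests to the hub, plus unbind-from-all.
; Relying on PostLogin limits it to offline single-player games; less restricted hooks require C++.
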(event EventBindMultipletoMultipleEvents
  (params (GameplayTags :type Gameplay%20Tag%20Container%20Structure) (ObjectsToBind :type Array%20of%20Object%20Object%20References))
  ;[0 0 0 1 35] Binding
  (Default|BindMultipletoMultiple (Variables|Default|GetEvent%20Dispatcher%20Hub%20Reference) GameplayTags ObjectsToBind))

(event EventBindMultipletoSingleEvent
  (params (GameplayTag :type Gameplay%20Tag%20Structure) (ObjectsToBind :type Array%20of%20Object%20Object%20References))
  ;[0 0 0 1 35] Binding
  (Default|BindMultipleObjectstoOneTag (Variables|Default|GetEvent%20Dispatcher%20Hub%20Reference) GameplayTag ObjectsToBind))

(event EventBindtoMultipleEvents
  (params (GameplayTags :type Gameplay%20Tag%20Container%20Structure) (ObjectToBind :type Object%20Object%20Reference))
  ;[0 0 0 1 35] Binding
  (Default|BindOnetoMultiple (Variables|Default|GetEvent%20Dispatcher%20Hub%20Reference) GameplayTags ObjectToBind))

(event EventUnbindfromAll
  (params (ObjectToUnbind :type Object%20Object%20Reference))
  ;[0 0 0 1 35] Unbinding
  (Default|UnbindfromAll (Variables|Default|GetEvent%20Dispatcher%20Hub%20Reference) ObjectToUnbind))

(event EventPostLogin
  (params (NewPlayer :type Player%20Controller%20Object%20Reference))
  ;[0 0 0 1 35] Due to the usage of OnPostLogin, this Blueprint is only usable in One-Player, Offline, Solo games.
  ; To use less restricted events, C++ is required.
  (bind _returnvalue (Game|SpawnActorfromClass "/EventDispatcherHub/Blueprints/BP_EDH_EventDispatcherHub.BP_EDH_EventDispatcherHub_C" (Math|Transform|MakeTransform "0, 0, 0" "0, 0, 0" "1.000000,1.000000,1.000000") "Undefined" "MultiplyWithRoot" 0 0))
  (Variables|Default|SetEvent%20Dispatcher%20Hub%20Reference _returnvalue))

(event EventBindtoSingleEvent
  (params (GameplayTag :type Gameplay%20Tag%20Structure) (ObjectToBind :type Object%20Object%20Reference))
  ;[0 0 0 1 35] Binding
  (Default|BindOneObjecttoOneTag (Variables|Default|GetEvent%20Dispatcher%20Hub%20Reference) GameplayTag ObjectToBind))

(event EventUnbindMultiplefromMultipleEvents
  (params (GameplayTags :type Gameplay%20Tag%20Container%20Structure) (ObjectsToUnbind :type Array%20of%20Object%20Object%20References))
  ;[0 0 0 1 35] Unbinding
  (Default|UnbindMultiplefromMultiple (Variables|Default|GetEvent%20Dispatcher%20Hub%20Reference) GameplayTags ObjectsToUnbind))

(event EventUnbindMultiplefromSingleEvent
  (params (GameplayTag :type Gameplay%20Tag%20Structure) (ObjectsToUnbind :type Array%20of%20Object%20Object%20References))
  ;[0 0 0 1 35] Unbinding
  (Default|UnbindMultiplefromOne (Variables|Default|GetEvent%20Dispatcher%20Hub%20Reference) GameplayTag ObjectsToUnbind))

(event EventUnbindfromMultipleEvents
  (params (GameplayTags :type Gameplay%20Tag%20Container%20Structure) (ObjectToUnbind :type Object%20Object%20Reference))
  ;[0 0 0 1 35] Unbinding
  (Default|UnbindOnefromMultiple (Variables|Default|GetEvent%20Dispatcher%20Hub%20Reference) GameplayTags ObjectToUnbind))

(event EventUnbindfromSingleEvent
  (params (GameplayTag :type Gameplay%20Tag%20Structure) (ObjectToUnbind :type Object%20Object%20Reference))
  ;[0 0 0 1 35] Unbinding
  (Default|UnbindOnefromOne (Variables|Default|GetEvent%20Dispatcher%20Hub%20Reference) GameplayTag ObjectToUnbind))

(event EventCallMultipleEvents
  (params (TagsToCall :type Gameplay%20Tag%20Container%20Structure) (CallingObject :type Object%20Object%20Reference))
  ;[0 0 0 1 35] Calling
  (Default|TryCallMultipleEvents (Variables|Default|GetEvent%20Dispatcher%20Hub%20Reference) TagsToCall CallingObject))

(event EventCallSingleEvent
  (params (TagToCall :type Gameplay%20Tag%20Structure) (CallingObject :type Object%20Object%20Reference))
  ;[0 0 0 1 35] Calling
  (Default|TryCallSingleEvent (Variables|Default|GetEvent%20Dispatcher%20Hub%20Reference) TagToCall CallingObject))

(fn ConstructionScript)