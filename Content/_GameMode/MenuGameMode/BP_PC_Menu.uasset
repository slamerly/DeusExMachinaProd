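; BP_PC_Menu is the menu player controller that routes Enhanced Input to the active menu.
; On BeginPlay it caches the first actor implementing BPI_Menu and adds the IMC_Menu mapping context.
; The navigate, enter and back input actions forward to that actor as BPI_Menu interface messages, so the controller holds no menu logic itself.
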(event Input|EnhancedActionEvents|EnhancedInputActionIA_MenuNav
  (params (ActionValue :type Float%20%28double-precision%29) (ElapsedSeconds :type Float%20%28double-precision%29) (TriggeredSeconds :type Float%20%28double-precision%29) (InputAction :type Input%20Action%20Object%20Reference :default "/Game/Inputs/InputsMenu/IA_MenuNav.IA_MenuNav"))
  (:Started
    (Class|BPIMenu|InputNav(Message) (Variables|Default|GetMenu) ActionValue)))

(event Input|EnhancedActionEvents|EnhancedInputActionIA_MenuEnter
  (params (ActionValue :type Boolean) (ElapsedSeconds :type Float%20%28double-precision%29) (TriggeredSeconds :type Float%20%28double-precision%29) (InputAction :type Input%20Action%20Object%20Reference :default "/Game/Inputs/InputsMenu/IA_MenuEnter.IA_MenuEnter"))
  (:Started
    (Class|BPIMenu|ButtonsActions(Message) (Variables|Default|GetMenu))))

(event Input|EnhancedActionEvents|EnhancedInputActionIA_MenuBack
  (params (ActionValue :type Boolean) (ElapsedSeconds :type Float%20%28double-precision%29) (TriggeredSeconds :type Float%20%28double-precision%29) (InputAction :type Input%20Action%20Object%20Reference :default "/Game/Inputs/InputsMenu/IA_MenuBack.IA_MenuBack"))
  (:Started
    (Class|BPIMenu|BacktoMenu(Message) (Variables|Default|GetMenu))))

(event EventBeginPlay
  (bind _self self)
  (bind _returnvalue (PlayerController|LocalPlayerSubsystems|GetEnhancedInputLocalPlayerSubsystem _self))
  (bind _outactors (Actor|GetAllActorswithInterface "/Game/Gameplay/Menu/BPI_Menu.BPI_Menu_C"))
  (Variables|Default|SetMenu (Utilities|Array|Get(acopy) _outactors))
  (Utilities|IsValid _returnvalue
    (:Is%20Valid
      (Input|AddMappingContext _returnvalue "/Game/Inputs/InputsMenu/IMC_Menu.IMC_Menu" 0 "(bIgnoreAllPressedKeysUntilRelease=True,bForceImmediately=False,bNotifyUserSettings=False)"))))

(fn ConstructionScript)