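; Game mode for single-player offline play that acts as a central access point for camera control and gameplay-tag events.
; OnPostLogin spawns the event dispatcher hub before BeginPlay so actors can register early; bind, unbind and call events forward to it.
; Camera events pass lens, mode, spline, data asset, shake, wiggle and hover changes to BP_DeusExCamera, which a macro finds lazily and caches.
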(event EventUpdateFocalLength
  (params (New%20Focal%20Length :type Float%20%28double-precision%29) (Switch%20Speed :type Float%20%28double-precision%29))
  ;[1 0.2816 0.4835 1 50] CAMERA
  (bind _camera (Utilities|CameraReference)
    (:Output
      (Variables|/Game/Camera/BP_DeusExCamera.BP_DeusExCamera_C|SetTarget%20Focal%20Length _camera New%20Focal%20Length)
      (Variables|/Game/Camera/BP_DeusExCamera.BP_DeusExCamera_C|SetFocal%20Length%20Switch%20Speed _camera Switch%20Speed))))

(event EventSetNewSpline
  (params (New%20Spline :type BP%20Deus%20Ex%20Camera%20Spline%20Object%20Reference) (ConstraintToSpline :type Boolean))
  ;[1 0.2816 0.4835 1 50] CAMERA
  (bind _camera (Utilities|CameraReference)
    (:Output
      (Default|SwitchSplinetoFollow _camera New%20Spline ConstraintToSpline))))

(event EventBindMultipletoMultipleEvents
  (params (GameplayTags :type Gameplay%20Tag%20Container%20Structure) (ObjectsToBind :type Array%20of%20Object%20Object%20References))
  ;[0 0 0 1 35] Binding
  (Default|BindMultipletoMultiple (Variables|Default|GetEvent%20Dispatcher%20Hub%20Reference) GameplayTags ObjectsToBind))

(event EventBindMultipletoSingleEvent
  (params (GameplayTag :type Gameplay%20Tag%20Structure) (ObjectsToBind :type Array%20of%20Object%20Object%20References))
  ;[0 0 0 1 35] Binding
  (Default|BindMultipleObjectstoOneTag (Variables|Default|GetEvent%20Dispatcher%20Hub%20Reference) GameplayTag ObjectsToBind))

(event EventBindtoMultipleEvents
  (params (GameplayTags :type Gameplay%20Tag%20Container%20Structure) (ObjectToBind :type Object%20Object%20Reference))
  ;[0 0 0 1 35] Binding
  (Default|BindOnetoMultiple (Variables|Default|GetEvent%20Dispatcher%20Hub%20Reference) GameplayTags ObjectToBind))

(event EventUnbindfromAll
  (params (ObjectToUnbind :type Object%20Object%20Reference))
  ;[0 0 0 1 35] Unbinding
  (Default|UnbindfromAll (Variables|Default|GetEvent%20Dispatcher%20Hub%20Reference) ObjectToUnbind))

(event EventSwitchCameraBehaviourMode
  (params (New%20Mode :type E_DeusExCameraModes%20Enum :default "NewEnumerator0"))
  ;[1 0.2816 0.4835 1 50] CAMERA
  (bind _camera (Utilities|CameraReference)
    (:Output
      (Variables|/Game/Camera/BP_DeusExCamera.BP_DeusExCamera_C|SetCurrent%20Camera%20Mode _camera New%20Mode))))

(event EventSwitchWiggleHoverData
  (params (New%20Wiggle%20Hover%20Data :type PDA%20Deus%20Ex%20Camera%20Wiggle%20and%20Hover%20Object%20Reference) (Hover%20Intensity%20Interp%20Speed :type Float%20%28double-precision%29) (Wiggle%20Intensity%20Interp%20Speed :type Float%20%28double-precision%29))
  ;[1 0.2816 0.4835 1 50] CAMERA
  (bind _camera (Utilities|CameraReference)
    (:Output
      (Default|SwitchHoverandWiggleData _camera New%20Wiggle%20Hover%20Data Hover%20Intensity%20Interp%20Speed Wiggle%20Intensity%20Interp%20Speed))))

(event EventEditShouldDebugBoolean
  (params (New%20Should%20Debug :type Boolean))
  ;[1 0.2816 0.4835 1 50] CAMERA
  (bind _camera (Utilities|CameraReference)
    (:Output
      (Variables|/Game/Camera/BP_DeusExCamera.BP_DeusExCamera_C|SetShould%20Debug _camera New%20Should%20Debug))))

(event EventSwitchSplineFollowDataAsset
  (params (New%20Data%20Asset :type PDA%20Deus%20Ex%20Camera%20Follow%20Spline%20Data%20Object%20Reference) (Movement%20Speed%20Interp%20Speed :type Float%20%28double-precision%29) (Rotation%20Speed%20Interp%20Speed :type Float%20%28double-precision%29))
  ;[1 0.2816 0.4835 1 50] CAMERA
  (bind _camera (Utilities|CameraReference)
    (:Output
      (Default|SwitchFollowSplineDataAsset _camera New%20Data%20Asset Movement%20Speed%20Interp%20Speed Rotation%20Speed%20Interp%20Speed))))

(event EventSwitchAct1DataAsset
  (params (New%20Data%20Asset :type PDA%20Deus%20Ex%20Camera%20Act%201%20Data%20Object%20Reference))
  ;[1 0.2816 0.4835 1 50] CAMERA
  (bind _camera (Utilities|CameraReference)
    (:Output
      (Variables|/Game/Camera/BP_DeusExCamera.BP_DeusExCamera_C|SetAct%201%20Data _camera New%20Data%20Asset))))

(event EventSwitchSplineSecondaryTarget
  (params (New%20Secondary%20Target :type Actor%20Object%20Reference))
  ;[1 0.2816 0.4835 1 50] CAMERA
  (bind _camera (Utilities|CameraReference)
    (:Output
      (Variables|/Game/Camera/BP_DeusExCamera.BP_DeusExCamera_C|SetCamera%20Secondary%20Target%20Point _camera New%20Secondary%20Target))))

(event EventPostLogin
  (params (NewPlayer :type Player%20Controller%20Object%20Reference))
  ;[0 0 0 1 35] Due to the usage of OnPostLogin, this Blueprint is only usable in One-Player, Offline, Solo games.
  ; To use less restricted events, C++ is required.
  (bind _returnvalue (Game|SpawnActorfromClass "/EventDispatcherHub/Blueprints/BP_EDH_EventDispatcherHub.BP_EDH_EventDispatcherHub_C" (Math|Transform|MakeTransform "0, 0, 0" "0, 0, 0" "1.000000,1.000000,1.000000") "Undefined" "MultiplyWithRoot" 0 0))
  (Variables|Default|SetEvent%20Dispatcher%20Hub%20Reference _returnvalue))

(event EventAddNewCameraShake
  (params (New%20Camera%20Shake%20Data :type PDA%20Deus%20Ex%20Camera%20Shake%20Object%20Reference))
  ;[1 0.2816 0.4835 1 50] CAMERA
  (bind _camera (Utilities|CameraReference)
    (:Output
      (Default|AddNewCameraShake _camera New%20Camera%20Shake%20Data))))

(event EventUpdateAperture
  (params (New%20Aperture :type Float%20%28double-precision%29) (Aperture%20Switch%20Speed :type Float%20%28double-precision%29))
  ;[1 0.2816 0.4835 1 50] CAMERA
  (bind _camera (Utilities|CameraReference)
    (:Output
      (Default|SwitchAperture _camera New%20Aperture Aperture%20Switch%20Speed))))

(event EventUpdateFocusSettings
  (params (New%20Focus%20Distance :type Float%20%28double-precision%29) (Focus%20Distance%20Switch%20Speed :type Float%20%28double-precision%29))
  ;[1 0.2816 0.4835 1 50] CAMERA
  (bind _camera (Utilities|CameraReference)
    (:Output
      (Default|SwitchFocusDistance _camera New%20Focus%20Distance Focus%20Distance%20Switch%20Speed))))

(event EventUpdateFilmbackSettings
  (params (New%20Filmback%20Settings :type Camera%20Filmback%20Settings%20Structure) (Filmback%20Switch%20Speed :type Float%20%28double-precision%29))
  ;[1 0.2816 0.4835 1 50] CAMERA
  (bind _camera (Utilities|CameraReference)
    (:Output
      (Default|SwitchFilmbackSettings _camera New%20Filmback%20Settings Filmback%20Switch%20Speed))))

(event EventSwitchAct1TargetLocation
  (params (New%20Target%20Location :type Vector :default "0, 0, 0"))
  ;[1 0.2816 0.4835 1 50] CAMERA
  (bind _camera (Utilities|CameraReference)
    (:Output
      (Variables|/Game/Camera/BP_DeusExCamera.BP_DeusExCamera_C|SetTarget%20Act%201%20Location _camera New%20Target%20Location))))

(event EventSetShouldHover
  (params (Should%20Hover :type Boolean))
  ;[1 0.2816 0.4835 1 50] CAMERA
  (bind _camera (Utilities|CameraReference)
    (:Output
      (Variables|/Game/Camera/BP_DeusExCamera.BP_DeusExCamera_C|SetShould%20Hover _camera Should%20Hover))))

(event EventSwitchPlayerWalkableStrictSpline
  (params (New%20Player%20Spline :type BP%20Player%20Walkable%20Spline%20Object%20Reference))
  ;[1 0.2816 0.4835 1 50] CAMERA
  (bind _camera (Utilities|CameraReference)
    (:Output
      (Variables|/Game/Camera/BP_DeusExCamera.BP_DeusExCamera_C|SetPlayer%20Movement%20Spline _camera New%20Player%20Spline))))

(event EventSetShouldCameraShake
  (params (Should%20Camera%20Shake :type Boolean))
  ;[1 0.2816 0.4835 1 50] CAMERA
  (bind _camera (Utilities|CameraReference)
    (:Output
      (Variables|/Game/Camera/BP_DeusExCamera.BP_DeusExCamera_C|SetShould%20Camera%20Shake _camera Should%20Camera%20Shake))))

(event EventSwitchStrictSplineDataAsset
  (params (New%20Data%20Asset :type PDA%20Deus%20Ex%20Camera%20Strict%20Spline%20Data%20Object%20Reference) (Movement%20Speed%20Interp%20Speed :type Float%20%28double-precision%29) (Rotation%20Speed%20Interp%20Speed :type Float%20%28double-precision%29))
  ;[1 0.2816 0.4835 1 50] CAMERA
  (bind _camera (Utilities|CameraReference)
    (:Output
      (Default|SwitchStrictSplineDataAsset _camera New%20Data%20Asset Movement%20Speed%20Interp%20Speed Rotation%20Speed%20Interp%20Speed))))

(event EventBindtoSingleEvent
  (params (GameplayTag :type Gameplay%20Tag%20Structure) (ObjectToBind :type Object%20Object%20Reference))
  ;[0 0 0 1 35] Binding
  (Default|BindOneObjecttoOneTag (Variables|Default|GetEvent%20Dispatcher%20Hub%20Reference) GameplayTag ObjectToBind))

(event EventSetShouldWiggle
  (params (Should%20Wiggle :type Boolean))
  ;[1 0.2816 0.4835 1 50] CAMERA
  (bind _camera (Utilities|CameraReference)
    (:Output
      (Variables|/Game/Camera/BP_DeusExCamera.BP_DeusExCamera_C|SetShould%20Wiggle _camera Should%20Wiggle))))

(event EventSwitchBoxRoamDataAsset
  (params (New%20Data%20Asset :type PDA%20Deus%20Ex%20Camera%20Box%20Roam%20Data%20Object%20Reference) (Movement%20Speed%20Interp%20Speed :type Float%20%28double-precision%29) (Rotation%20Speed%20Interp%20Speed :type Float%20%28double-precision%29))
  ;[1 0.2816 0.4835 1 50] CAMERA
  (bind _camera (Utilities|CameraReference)
    (:Output
      (Default|SwitchBoxRoamDataAsset _camera New%20Data%20Asset Movement%20Speed%20Interp%20Speed Rotation%20Speed%20Interp%20Speed))))

(event EventUnbindMultiplefromMultipleEvents
  (params (GameplayTags :type Gameplay%20Tag%20Container%20Structure) (ObjectsToUnbind :type Array%20of%20Object%20Object%20References))
  ;[0 0 0 1 35] Unbinding
  (Default|UnbindMultiplefromMultiple (Variables|Default|GetEvent%20Dispatcher%20Hub%20Reference) GameplayTags ObjectsToUnbind))

(event EventUnbindMultiplefromSingleEvent
  (params (GameplayTag :type Gameplay%20Tag%20Structure) (ObjectsToUnbind :type Array%20of%20Object%20Object%20References))
  ;[0 0 0 1 35] Unbinding
  (Default|UnbindMultiplefromOne (Variables|Default|GetEvent%20Dispatcher%20Hub%20Reference) GameplayTag ObjectsToUnbind))

(event EventUnbindfromMultipleEvents
  (params (GameplayTags :type Gameplay%20Tag%20Container%20Structure) (ObjectToUnbind :type Object%20Object%20Reference))
  ;[0 0 0 1 35] Unbinding
  (Default|UnbindOnefromMultiple (Variables|Default|GetEvent%20Dispatcher%20Hub%20Reference) GameplayTags ObjectToUnbind))

(event EventUnbindfromSingleEvent
  (params (GameplayTag :type Gameplay%20Tag%20Structure) (ObjectToUnbind :type Object%20Object%20Reference))
  ;[0 0 0 1 35] Unbinding
  (Default|UnbindOnefromOne (Variables|Default|GetEvent%20Dispatcher%20Hub%20Reference) GameplayTag ObjectToUnbind))

(event EventCallMultipleEvents
  (params (TagsToCall :type Gameplay%20Tag%20Container%20Structure) (CallingObject :type Object%20Object%20Reference))
  ;[0 0 0 1 35] Calling
  (Default|TryCallMultipleEvents (Variables|Default|GetEvent%20Dispatcher%20Hub%20Reference) TagsToCall CallingObject))

(event EventCallSingleEvent
  (params (TagToCall :type Gameplay%20Tag%20Structure) (CallingObject :type Object%20Object%20Reference))
  ;[0 0 0 1 35] Calling
  (Default|TryCallSingleEvent (Variables|Default|GetEvent%20Dispatcher%20Hub%20Reference) TagToCall CallingObject))

(fn ConstructionScript)