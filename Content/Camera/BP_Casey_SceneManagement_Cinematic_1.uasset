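; Scripted cinematic manager that plays the Juliet spear scene and hands off to the theater level.
; On BeginPlay, chained Timelines lerp hard-coded transforms to open doors, fly in three spears, then retract two and drag Juliet away on the third.
; A separate event topples the house alongside the spear retraction.
; It then reveals the theater, raises the player pawn, pulls the camera spline back while curtains close, and loads LVL_TheaterScene_Base.
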(event Custom|Housefallingg
  (bind _housefalling (Timeline|HouseFalling PlayFromStart)
    (:Update
      (Transformation|SetActorRotation (Variables|Default|GetHouseRotator) (Math|Rotator|MakeRotator 0.0 (Math|Float|Lerp 0.0 -9e+01 _housefalling) 0.0))
      (Transformation|SetActorRelativeRotation (Variables|Default|Get1stDoorsToOpen) (Math|Rotator|MakeRotator 0.0 0.0 (Math|Float|Lerp 105.0 1.8e+02 _housefalling)))
      (Transformation|SetActorRelativeRotation (Variables|Default|Get2sdDoorsToOpen) (Math|Rotator|MakeRotator 0.0 0.0 (Math|Float|Lerp 75.0 0.0 _housefalling))))))

(event EventBeginPlay
  (bind _returnvalue (Game|Player|GetPlayerPawn 0))
  (bind _2sdcurtain (Variables|Default|Get2sdCurtain))
  (bind _1stcurtain (Variables|Default|Get1stCurtain))
  (bind _cameraspline (Variables|Default|GetCameraSpline))
  (bind _returnvalue_2 (Transformation|GetActorLocation _2sdcurtain))
  (bind _returnvalue_3 (Transformation|GetActorLocation _1stcurtain))
  (bind _returnvalue_4 (Transformation|GetActorLocation _cameraspline))
  (bind _returnvalue_5 (Transformation|GetActorLocation _returnvalue))
  (Utilities|FlowControl|Delay (Variables|Default|GetDelayDurationBeforeOpeningDoor))
  (bind _openingdoors (Timeline|OpeningDoors PlayFromStart)
    (:Update
      (Transformation|SetActorRotation (Variables|Default|Get1stDoorsToOpen) (Math|Rotator|MakeRotator 0.0 0.0 (Math|Float|Lerp 0.0 (Variables|Default|Get1stDoorsFinalRotationZ) _openingdoors)))
      (Transformation|SetActorRotation (Variables|Default|Get2sdDoorsToOpen) (Math|Rotator|MakeRotator 0.0 0.0 (Math|Float|Lerp -1.8e+02 (* (Variables|Default|Get2sdDoorsFinalRotationZ) -1.0) _openingdoors))))
    (:Finished
      (Utilities|FlowControl|Delay 2.0)
      (Rendering|SetActorHiddenInGame (Variables|Default|Get1stSpear) false)
      (Rendering|SetActorHiddenInGame (Variables|Default|Get2sdSpear) false)
      (Rendering|SetActorHiddenInGame (Variables|Default|Get3thSpear) false)
      (bind _spearjuliet (Timeline|SpearJuliet PlayFromStart)
        (:Update
          (Transformation|SetActorRelativeLocation (Variables|Default|Get1stSpear) (Math|Vector|MakeVector 7e+01 (Math|Float|Lerp -1415.0 -535.0 _spearjuliet) (Math|Float|Lerp 1685.0 4.3e+02 _spearjuliet)))
          (Transformation|SetActorRelativeLocation (Variables|Default|Get2sdSpear) (Math|Vector|MakeVector 7e+01 (Math|Float|Lerp -115.0 -3.9e+02 _spearjuliet) (Math|Float|Lerp 1.24e+03 485.0 _spearjuliet)))
          (Transformation|SetActorRelativeLocation (Variables|Default|Get3thSpear) (Math|Vector|MakeVector 7e+01 (Math|Float|Lerp -1455.0 -825.0 _spearjuliet) 315.0)))
        (:Finished
          (CallFunction|Housefallingg)
          (Utilities|FlowControl|Delay 1.0)
          (bind _removespear (Timeline|RemoveSpear PlayFromStart)
            (:Update
              (Transformation|SetActorRelativeLocation (Variables|Default|Get1stSpear) (Math|Vector|MakeVector 7e+01 (Math|Float|Lerp -535.0 -1415.0 _removespear) (Math|Float|Lerp 4.3e+02 1685.0 _removespear)))
              (Transformation|SetActorRelativeLocation (Variables|Default|Get2sdSpear) (Math|Vector|MakeVector 9e+01 (Math|Float|Lerp -3.9e+02 -115.0 _removespear) (Math|Float|Lerp 485.0 1.24e+03 _removespear))))
            (:Finished
              (bind _dragjuliet (Timeline|DragJuliet PlayFromStart)
                (:Update
                  (Transformation|SetActorRelativeLocation (Variables|Default|Get3thSpear) (Math|Vector|MakeVector 7e+01 (Math|Float|Lerp -825.0 -1455.0 _dragjuliet) 315.0))
                  (Transformation|SetActorRelativeLocation (Variables|Default|GetJuliet) (Math|Vector|MakeVector 9e+01 (Math|Float|Lerp -4.6e+02 -1.13e+03 _dragjuliet) 5e+01)))
                (:Finished
                  (Actor|DestroyActor (Variables|Default|GetJuliet))
                  (Actor|DestroyActor (Variables|Default|Get3thSpear))
                  (Actor|DestroyActor (Variables|Default|Get2sdSpear))
                  (Actor|DestroyActor (Variables|Default|Get1stSpear))
                  (Rendering|SetActorHiddenInGame (Variables|Default|GetTheater) false)
                  (Rendering|SetActorHiddenInGame (Variables|Default|GetTheaterText) false)
                  (Rendering|SetActorHiddenInGame (Variables|Default|Get1stCurtain) false)
                  (Rendering|SetActorHiddenInGame (Variables|Default|Get2sdCurtain) false)
                  (Transformation|SetActorLocation _returnvalue (Math|Vector|MakeVector (.x _returnvalue_5) (.y _returnvalue_5) (+ (.z _returnvalue_5) 1e+03)) false false)
                  (bind (_direction _cameragoesbac _curtain) (Timeline|CameraGoesBack PlayFromStart)
                    (:Update
                      (Transformation|SetActorLocation _cameraspline (Math|Vector|MakeVector (Math|Float|Lerp -2.65e+03 -5e+03 _cameragoesbac) (.y _returnvalue_4) (.z _returnvalue_4)) false false)
                      (Transformation|SetActorLocation (Variables|Default|Get1stCurtain) (Math|Vector|MakeVector (.x _returnvalue_3) (Math|Float|Lerp -1.65e+03 -1e+02 _curtain) (.z _returnvalue_3)) false false)
                      (Transformation|SetActorLocation (Variables|Default|Get2sdCurtain) (Math|Vector|MakeVector (.x _returnvalue_2) (Math|Float|Lerp 3.4e+03 1.9e+03 _curtain) (.z _returnvalue_2)) false false))
                    (:Finished
                      (Utilities|FlowControl|Delay 2.0)
                      (Game|OpenLevel(byName) "LVL_TheaterScene_Base"))))))))))))

(fn ConstructionScript)