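; Test actor that changes the automatic rotation settings of a linked rotation support when a button is used.
; On BeginPlay it binds to the Button's MovSys button-used event.
; On the first use, it finds the RotationBehaviorAutomatic component on the RotationSupportAutomatic actor and applies ChangeAutoRotValues.
; A ChangeDone flag makes the change one-shot once it succeeds.
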(event Custom|OnButtonUsed
  (bind _rotationsupportautomatic (Variables|Default|GetRotationSupportAutomatic))
  (bind _returnvalue (Actor|GetComponentbyClass _rotationsupportautomatic "/Script/DeusExMachina.RotationBehaviorAutomatic"))
  (if (not (Variables|Default|GetbChangeDone))
    (Utilities|IsValid _rotationsupportautomatic
      (:Is%20Valid
        (Utilities|IsValid _returnvalue
          (:Is%20Valid
            (Class|RotationBehaviorAutomatic|ChangeAutomaticRotationValues _returnvalue (Variables|Default|GetChangeAutoRotValues))
            (Variables|Default|SetbChangeDone true)))))))

(event EventBeginPlay
  (bind _button (Variables|Default|GetButton))
  (Utilities|IsValid _button
    (:Is%20Valid
      (EventDispatchers|AssignOnMovSysButtonUsed _button (delegate Custom|OnButtonUsed)))))

(event Collision|EventActorBeginOverlap
  (params (OtherActor :type Actor%20Object%20Reference)))

(event EventTick
  (params (DeltaSeconds :type Float%20%28single-precision%29)))

(fn ConstructionScript)