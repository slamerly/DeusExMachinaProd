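; BP_TestInteraction is a test actor for the interaction system that prints a debug message with its own name when interacted with.
; It always reports that it can be interacted with and that the interaction is not heavy.
; The interaction tooltip position comes from the world location of its InteractTooltip component.
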(event EventBeginPlay)

(event Collision|EventActorBeginOverlap
  (params (OtherActor :type Actor%20Object%20Reference)))

(event EventTick
  (params (DeltaSeconds :type Float%20%28single-precision%29)))

(event EventInteraction
  (Development|PrintText (Utilities|Text|FormatText "Test Interaction. | Object {name}" (Utilities|GetDisplayName self))))

(fn ConstructionScript)

(fn CanInteract
  (return true))

(fn GetInteractableTooltipPosition
  (return (Transformation|GetWorldLocation (Variables|Default|GetInteractTooltip))))

(fn IsInteractionHeavy
  (return false))