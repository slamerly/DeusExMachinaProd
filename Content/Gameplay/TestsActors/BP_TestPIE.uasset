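; BP_TestPIE is an interactable test actor, apparently meant to show on a TextRender whether the game runs in PIE or a build.
; Its Interaction event branches on a hardcoded true, so it always displays "PIE"; the IsInEditor check is left unconnected.
; The interaction functions report it as always interactable, one-sided and light, with the tooltip at the Scene component's location.
; String file save and load nodes are present but never run.
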(event EventBeginPlay)

(event Collision|EventActorBeginOverlap
  (params (OtherActor :type Actor%20Object%20Reference)))

(event EventTick
  (params (DeltaSeconds :type Float%20%28single-precision%29)))

(event EventInteraction
  (bind _textrender (Variables|Default|GetTextRender))
  (if true
    (Rendering|Components|TextRender|SetText _textrender (Utilities|Text|MakeLiteralText "PIE"))
    (else
      (Rendering|Components|TextRender|SetText _textrender (Utilities|Text|MakeLiteralText "Build")))))

(fn ConstructionScript)

(fn CanInteract
  (return true))

(fn GetInteractableFocusActor
  (return 0))

(fn GetInteractableTooltipPosition
  (return (Transformation|GetWorldLocation (Variables|Default|GetScene))))

(fn IsInteractableBothSides
  (return false))

(fn IsInteractionHeavy
  (return false))