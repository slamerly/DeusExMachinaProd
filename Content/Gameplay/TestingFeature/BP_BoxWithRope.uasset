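; BP_BoxWithRope is a test actor: a cube with a cable component that ties to another actor and lets go when that actor gets too far away.
; On BeginPlay the cable's end attaches to ActorToAttach.
; Each Tick prints the signed X offset from the cube to the attached actor and turns off AttachEnd once it exceeds a fixed threshold, with no reattach logic.
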(event EventBeginPlay
  (Class|CableComponent|SetAttachEndto (Variables|Default|GetCable) (Variables|Default|GetActorToAttach) "None" "None"))

(event EventTick
  (params (DeltaSeconds :type Float%20%28single-precision%29))
  (bind _cable (Variables|Default|GetCable))
  (bind _cube (Variables|Default|GetCube))
  (bind _returnvalue (Class|CableComponent|GetAttachedActor _cable))
  (bind _returnvalue_2 (Transformation|GetWorldLocation _cube))
  (bind _returnvalue_3 (Transformation|GetActorLocation _returnvalue))
  (bind _returnvalue_4 (- _returnvalue_3 _returnvalue_2))
  (Development|PrintString (Utilities|String|ToString(Float) (.x _returnvalue_4)))
  (if (> (.x _returnvalue_4) 4.5e+02)
    (Variables|/Script/CableComponent.CableComponent|SetbAttachEnd (Variables|Default|GetCable) false)))

(fn ConstructionScript)