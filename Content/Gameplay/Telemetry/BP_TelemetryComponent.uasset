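; Playtest telemetry component that records time spent between checkpoints and saves it as CSV under the project's Saved/PlaytestTelemetry folder.
; Each save writes a separate timestamped file, tagged PIE or Build, with user name, date, checkpoint index and elapsed time.
; Saves fire on each new checkpoint, level transition, quit, PIE end or debug key U.
; It binds to the all-candles-off chandelier event, but no handler appears here.
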(event EventEndPlay
  (params (EndPlayReason :type EEndPlayReason%20Enum :default "Destroyed"))
  (switch Utilities|FlowControl|Switch|SwitchonEEndPlayReason EndPlayReason
    (:LevelTransition
      _)
    (:EndPlayInEditor
      _)
    (:Quit
      _))
  (CallFunction|ParseandSaveAllData))

(event EventBeginPlay
  (CallFunction|BindtoMultipleGameplayEvents "(GameplayTags=((TagName=\"Event.Chandelier.AllCandlesOff\")))" self)
  (Utilities|FlowControl|DelayUntilNextTick)
  (bind _output_get (Variables|Default|SetOwner (Components|GetOwner)))
  (Variables|Default|SetTimeAtLastCheckpoint (Actor|GetGameTimeSinceCreation _output_get)))

(event Input|KeyboardEvents|DebugKeyU
  (params (Key :type Key%20Structure) (ActionValue :type Input%20Action%20Value%20Structure))
  (:Pressed
    (CallFunction|ParseandSaveAllData)))

(fn ParseandSaveAllData
  (bind _returnvalue (Math|DateTime|Now))
  (Variables|Default|SetDataToSave "")
  (Utilities|FlowControl|Sequence
    (:then_0
      ;[1 1 1 0.33] TimeSinceLastCheckpoint
      (bind _owner (Variables|Default|GetOwner)
        (:then
          (Variables|Default|SetGameTime (- (Actor|GetGameTimeSinceCreation _owner) (Variables|Default|GetTimeAtLastCheckpoint)))
          (Variables|Default|SetTimeAtLastCheckpoint (Actor|GetGameTimeSinceCreation (Variables|Default|GetOwner))))
        (:else)))
    (:then_1
      ;[1 1 1 0.33] Computer Session Name
      (CallFunction|AppendData (Utilities|Platform|GetPlatformUserName))
      ;[1 1 1 0.33] Date & Time
      (CallFunction|AppendData (Utilities|String|Replace (Utilities|String|ToString(Text) (Class|KismetTextLibrary|AsDateTimeDateTime (Math|DateTime|Now))) ","))
      ;[1 1 1 0.33] Checkpoint Number
      (CallFunction|AppendData (Utilities|String|ToString(Integer) (Variables|Default|GetCurrentCheckpointIndex)))
      ;[1 1 1 0.33] Game Since Checkpoint
      (CallFunction|AppendData (Utilities|String|ToString(Float) (Variables|Default|GetGameTime))))
    (:then_2
      (Class|MeasurementUtility|SaveStringasFile (Variables|Default|GetDataToSave) (Utilities|String|Append (Class|BlueprintPathsLibrary|ProjectSavedDir) "PlaytestTelemetry/" (Utilities|String|SelectString "PIE" "Build" (Class|MeasurementUtility|IsinEditor)) "_Data_" (Utilities|String|ToString(Text) (Utilities|Text|FormatText "{day}-{month}_{hour}-{minute}-{seconds}" (Utilities|Text|ToText(Integer) (.day _returnvalue) false true 2) (Utilities|Text|ToText(Integer) (.month _returnvalue) false true 2) (Utilities|Text|ToText(Integer) (.hour _returnvalue) false true 2) (Utilities|Text|ToText(Integer) (.minute _returnvalue) false true 2) (Utilities|Text|ToText(Integer) (.second _returnvalue) false true 2))) "_Checkpoint" (Utilities|String|ToString(Integer) (Variables|Default|GetCurrentCheckpointIndex)) ".csv"))
      (CallFunction|ClearAllData))))

(fn AppendData
  (params (Data :type String))
  (Variables|Default|SetDataToSave (Utilities|String|Append (Variables|Default|GetDataToSave) Data ",")))

(fn ClearAllData
  (Variables|Default|SetDataToSave ""))

(fn ReceiveNewCheckpoint
  (params (CheckpointIndex :type Integer))
  (CallFunction|ParseandSaveAllData)
  (Variables|Default|SetCurrentCheckpointIndex CheckpointIndex))