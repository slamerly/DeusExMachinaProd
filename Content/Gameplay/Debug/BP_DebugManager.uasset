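; BP_DebugManager is a debug toggle actor that opens and closes the debug menu from a debug key press.
; Each press flips its GamePaused flag, pausing or resuming the game and switching between game-only and game-and-UI input with the mouse cursor hidden or shown.
; It reaches the menu through the first player controller's HUD, calling enable or disable on the debug menu message object.
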(event EventBeginPlay)

(event Input|KeyboardEvents|DebugKey²
  (params (Key :type Key%20Structure :default "None") (ActionValue :type Input%20Action%20Value%20Structure))
  (bind _returnvalue (Game|GetPlayerController 0))
  (bind _returnvalue_2 (Game|GetPlayerController 0))
  (:Pressed
    (if (Variables|Default|GetGamePaused)
      (Variables|Default|SetGamePaused false)
      (Game|SetGamePaused false)
      (Input|SetInputModeGameOnly _returnvalue false)
      (Variables|/Script/Engine.PlayerController|SetbShowMouseCursor _returnvalue false)
      (bind _debugmenu (Class|BPIHUD|GetDebugMenu(Message) (HUD|GetHUD _returnvalue)))
      (Default|DisableDebugMenu _debugmenu)
      (else
        (Variables|Default|SetGamePaused true)
        (Game|SetGamePaused true)
        (Input|SetInputModeGameandUI _returnvalue_2 0 "LockOnCapture" false false)
        (Variables|/Script/Engine.PlayerController|SetbShowMouseCursor _returnvalue_2 true)
        (bind _debugmenu_2 (Class|BPIHUD|GetDebugMenu(Message) (HUD|GetHUD _returnvalue_2)))
        (Default|EnableDebugMenu _debugmenu_2)))))

(fn ConstructionScript)