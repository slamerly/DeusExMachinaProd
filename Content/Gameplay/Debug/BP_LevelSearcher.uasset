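; BP_LevelSearcher is a debug Blueprint that lists the map assets known to the Asset Registry.
; It queries the registry for World class assets, including subclasses, then prints the count and each package name on screen, or a "Nothing Found" message if the query fails.
; The search runs on BeginPlay when a flag is set, or whenever the numpad five debug key is pressed.
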(event EventBeginPlay
  (if (Variables|Default|GetShould%20Debug%20on%20Begin%20Play)
    (bind (_outassetdata _returnvalue) (Class|AssetRegistry|GetAssetsbyClass (Class|AssetRegistryHelpers|GetAssetRegistry) (Class|KismetSystemLibrary|GetClassTopLevelAssetPath "/Script/Engine.World") true))
    (if _returnvalue
      (Development|PrintString (Utilities|String|ToString(Integer) (Utilities|Array|Length _outassetdata)) true true "(R=1.000000,G=1.000000,B=0.000000,A=1.000000)" 5e+01)
      (for _array_element _outassetdata
        (Development|PrintText (Utilities|Text|FormatText "Map Package Name: {pn}" (.PackageName (Utilities|Struct|BreakAssetData _array_element))) true true "(R=0.000000,G=0.660000,B=1.000000,A=1.000000)" 5e+04))
      (else
        (Development|PrintString "Nothing Found")))))

(event Input|KeyboardEvents|DebugKeyNumPadFive
  (params (Key :type Key%20Structure :default "None") (ActionValue :type Input%20Action%20Value%20Structure))
  (:Pressed
    (bind (_outassetdata _returnvalue) (Class|AssetRegistry|GetAssetsbyClass (Class|AssetRegistryHelpers|GetAssetRegistry) (Class|KismetSystemLibrary|GetClassTopLevelAssetPath "/Script/Engine.World") true))
    (if _returnvalue
      (Development|PrintString (Utilities|String|ToString(Integer) (Utilities|Array|Length _outassetdata)) true true "(R=1.000000,G=1.000000,B=0.000000,A=1.000000)" 5e+01)
      (for _array_element _outassetdata
        (Development|PrintText (Utilities|Text|FormatText "Map Package Name: {pn}" (.PackageName (Utilities|Struct|BreakAssetData _array_element))) true true "(R=0.000000,G=0.660000,B=1.000000,A=1.000000)" 5e+04))
      (else
        (Development|PrintString "Nothing Found")))))

(fn ConstructionScript)