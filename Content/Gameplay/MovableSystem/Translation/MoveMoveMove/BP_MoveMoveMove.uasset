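; Moving platform that slides between a topmost and a bottommost point, accelerating toward the bottom up to a max speed with speed-scaled Perlin noise shaking its height.
; The construction script places endpoint markers and stretches and rolls a thin midway cube along the path, whose rotation the platform copies on BeginPlay.
; Tick forces the falling state every frame, leaving the rising branch unreachable, and the wheel-control binding is disconnected.
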(event Custom|OnWheelRotated
  (params (ControlValue :type Float%20%28single-precision%29) (TriggeredClamp :type Boolean))
  (Variables|Falling|SetisFalling false))

(event EventTick
  (params (DeltaSeconds :type Float%20%28single-precision%29))
  (bind _current_normalized_progress (Variables|Rising|GetCurrent%20Normalized%20Progress))
  (Variables|Falling|SetisFalling true)
  (if (Variables|Falling|GetisFalling)
    ;[0.4906 0.3027 1] Accelerate Falling !!
    (CallFunction|IncreaseValueFloatClamped (Variables|Falling|GetCurrentFallingSpeed) (* (Variables|Falling|GetFallingAcceleration) (Utilities|Time|GetWorldDeltaSeconds)) 0.0 (Variables|Falling|GetMaxFallingSpeed))
    ;[1 0.28 0.9833] Update Location
    (CallFunction|IncreaseValueFloatClamped (Variables|Rising|GetCurrent%20Normalized%20Progress) (* (Variables|Falling|GetCurrentFallingSpeed) (Utilities|Time|GetWorldDeltaSeconds)) 0.0 1.0)
    (else
      ;[1 0.28 0.9833] Update Location
      (CallFunction|DecreaseValueFloatClamped (Variables|Rising|GetCurrent%20Normalized%20Progress) (* (Variables|Rising|GetRisingSpeed) (Utilities|Time|GetWorldDeltaSeconds)) 0.0 1.0)))
  (Transformation|SetRelativeLocation (Variables|Default|GetPlatform) (+ (Math|Vector|Lerp(Vector) (Variables|Default|GetTopmost%20Location) (Variables|Default|GetBottommost%20Location) _current_normalized_progress) (Math|Vector|MakeVector 0.0 0.0 (* (Class|KismetMathLibrary|PerlinNoise1D (* _current_normalized_progress 2e+02 (Variables|Falling|GetCurrentFallingSpeed))) 85.0 (Variables|Falling|GetCurrentFallingSpeed)))) false false))

(event EventBeginPlay
  ;[1 1 1] Initialize Wall rotation to be parallel with the descent
  (Transformation|SetRelativeRotation (Variables|Default|GetPlatform) (Variables|/Script/Engine.SceneComponent|GetRelativeRotation (Variables|Default|GetSmallMidwayCube)) false false)
  (Variables|Rising|SetCurrent%20Normalized%20Progress (Variables|Default|GetStarting%20Lerp)))

(fn ConstructionScript
  (bind _topmost_location (Variables|Default|GetTopmost%20Location))
  (bind _bottommost_location (Variables|Default|GetBottommost%20Location))
  (bind _returnvalue (- _topmost_location _bottommost_location))
  (Transformation|SetRelativeLocation (Variables|Default|GetTopMostReference) (Variables|Default|GetTopmost%20Location) false false)
  (Transformation|SetRelativeLocation (Variables|Default|GetBottomMostReference) (Variables|Default|GetBottommost%20Location) false false)
  ;[1 1 1] Edit Roll rotation & Y Scale for length
  (Transformation|SetRelativeTransform (Variables|Default|GetSmallMidwayCube) (Math|Transform|MakeTransform (Math|Vector|Lerp(Vector) (Variables|Default|GetTopmost%20Location) (Variables|Default|GetBottommost%20Location) 0.5) (Math|Rotator|MakeRotator (* (Class|KismetMathLibrary|DegAtan (/ (.z _returnvalue) (.y _returnvalue))) -1.0) 0.0 0.0) (Math|Vector|MakeVector 0.03 (/ (Math|Vector|VectorLength (- (Variables|Default|GetTopmost%20Location) (Variables|Default|GetBottommost%20Location))) 1e+02) 0.03)) false false))