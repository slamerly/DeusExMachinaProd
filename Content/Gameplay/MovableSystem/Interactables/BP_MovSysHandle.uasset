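; Interactable handle for the movable system that shows interaction feedback by changing its material.
; The start and stop feedback events pass the interact or non-interact material to SetMaterialOnHandle, which applies it to both handle visual components.
; GetInteractableTooltipPosition returns the world location of the TooltipPos component to position the tooltip.
; The Blueprint contains no movement logic, only this visual feedback and tooltip placement.
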(event EventBeginPlay)

(event Collision|EventActorBeginOverlap
  (params (OtherActor :type Actor%20Object%20Reference)))

(event EventTick
  (params (DeltaSeconds :type Float%20%28single-precision%29)))

(event EventHandleStartFeedback
  (CallFunction|SetMaterialonHandle (Variables|HandleVisual|GetMaterialInteract)))

(event EventHandleStopFeedback
  (CallFunction|SetMaterialonHandle (Variables|HandleVisual|GetMaterialNonInteract)))

(fn ConstructionScript)

(fn GetInteractableTooltipPosition
  (return (Transformation|GetWorldLocation (Variables|Default|GetTooltipPos))))

(fn SetMaterialonHandle
  (params (Material :type Material%20Interface%20Object%20Reference))
  (Rendering|Material|SetMaterial (Variables|Default|GetHandleVisual) 0 Material)
  (Rendering|Material|SetMaterial (Variables|Default|GetHandleVisual1) 0 Material))