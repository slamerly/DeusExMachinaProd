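; Interactable notched selector lever for the movable system that shows which linked rotation and translation supports are currently selected.
; Feedback events swap the lever material for interaction and rotate it between notches, easing progress with a float curve across a centred angular range.
; On begin-play feedback and each selection update, it turns the selected visual on or off for every linked support.
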(event Custom|OnMovSysSelectorControlUpdated_Event
  (params (Selection :type Integer))
  (CallFunction|SetSelectedVisualonSupports))

(event EventBeginPlay)

(event Collision|EventActorBeginOverlap
  (params (OtherActor :type Actor%20Object%20Reference)))

(event EventTick
  (params (DeltaSeconds :type Float%20%28single-precision%29)))

(event EventSelectorStartFeedback
  (Rendering|Material|SetMaterial (Variables|Default|GetLever) 0 (Variables|SelectorVisual|GetMaterialInteract)))

(event EventSelectorStopFeedback
  (Rendering|Material|SetMaterial (Variables|Default|GetLever) 0 (Variables|SelectorVisual|GetMaterialNonInteract)))

(event EventSelectorBeginPlayFeedback
  (Utilities|FlowControl|Sequence
    (:then_0
      (CallFunction|RotateSelectorLever (Class|MovSysSelector|GetCurrentNotch) 0.0))
    (:then_1
      (CallFunction|SetSelectedVisualonSupports))
    (:then_2
      (EventDispatchers|AssignOnMovSysSelectorControlUpdated (delegate Custom|OnMovSysSelectorControlUpdated_Event)))))

(event EventSelectorUpdateFeedback
  (params (NotchProgressPercent :type Float%20%28single-precision%29) (NotchProgressTo :type Integer))
  (CallFunction|RotateSelectorLever (Class|MovSysSelector|GetCurrentNotch) NotchProgressPercent NotchProgressTo))

(fn ConstructionScript)

(fn GetInteractableTooltipPosition
  (return (Transformation|GetWorldLocation (Variables|Default|GetTooltipPos))))

(fn RotateSelectorLever
  (params (Notch :type Integer) (Progress :type Float%20%28double-precision%29) (ProgressToNotch :type Integer))
  (Utilities|FlowControl|Sequence
    (:then_0
      (LocalVariables|SetComputedProgress (+ (Math|Conversions|ToFloat(Integer) Notch) (* (Math|Curves|GetFloatValue (Variables|Default|GetSelectorFeedbackCurve) Progress) ProgressToNotch))))
    (:then_1
      (Transformation|SetRelativeRotation (Variables|Default|GetLever) (Math|Rotator|MakeRotator -9e+01 0.0 (- (* (LocalVariables|GetComputedProgress) (/ (Variables|Default|GetSelectorFeedbackAmplitude) (- (Variables|Default|GetNotchNumber) 1))) (/ (Variables|Default|GetSelectorFeedbackAmplitude) 2.0))) false false))))

(fn SetSelectedVisualonSupports
  (bind (_linkedrotsupportsselected _linkedtranssupportsselected) (Class|MovSysSelector|GetLinkedSupportsCurrentlySelected))
  (Utilities|FlowControl|Sequence
    (:then_0
      (for _array_element _linkedrotsupportsselected
        (bind _asbp_rotation_support_v_1 (Utilities|Casting|CastToBP_RotationSupport_v1 (.rotationsupport _array_element)))
        (Default|SetSelectedVisual _asbp_rotation_support_v_1 true)))
    (:then_1
      (for _array_element_2 _linkedtranssupportsselected
        (bind _asbp_translation_support_v_2 (Utilities|Casting|CastToBP_TranslationSupport_v2 (.translationsupport _array_element_2)))
        (Default|SetSelectedVisual _asbp_translation_support_v_2 true)))
    (:then_2
      (bind (_linkedrotsupportsselected_2 _linkedtranssupportsselected_2) (Class|MovSysSelector|GetLinkedSupportsCurrentlyNotSelected))
      (Utilities|FlowControl|Sequence
        (:then_0
          (for _array_element_3 _linkedrotsupportsselected_2
            (bind _asbp_rotation_support_v_1_2 (Utilities|Casting|CastToBP_RotationSupport_v1 (.rotationsupport _array_element_3)))
            (Default|SetSelectedVisual _asbp_rotation_support_v_1_2 false)))
        (:then_1
          (for _array_element_4 _linkedtranssupportsselected_2
            (bind _asbp_translation_support_v_2_2 (Utilities|Casting|CastToBP_TranslationSupport_v2 (.translationsupport _array_element_4)))
            (Default|SetSelectedVisual _asbp_translation_support_v_2_2 false)))))))