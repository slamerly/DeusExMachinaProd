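; BP_MovSysWheel is an interactable wheel control in the movable system, handling the visual feedback while it is used.
; Control feedback yaws the wheel mesh by the control value scaled by delta time and a visual speed.
; Start and stop feedback swap the wheel and its eight handles between interact and non-interact materials.
; A TooltipPos component supplies the world position of the interaction tooltip.
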(event EventBeginPlay)

(event Collision|EventActorBeginOverlap
  (params (OtherActor :type Actor%20Object%20Reference)))

(event EventTick
  (params (DeltaSeconds :type Float%20%28single-precision%29)))

(event EventWheelControlFeedback
  (params (ControlValue :type Float%20%28single-precision%29))
  (Transformation|AddLocalRotation (Variables|Default|GetWheel) (Math|Rotator|MakeRotator 0.0 0.0 (* ControlValue (Utilities|Time|GetWorldDeltaSeconds) (Variables|WheelVisual|GetWheelVisualSpeed))) false false))

(event EventWheelStartFeedback
  (CallFunction|SetMaterialonWheel (Variables|WheelVisual|GetMaterialInteract)))

(event EventWheelStopFeedback
  (CallFunction|SetMaterialonWheel (Variables|WheelVisual|GetMaterialNonInteract)))

(fn ConstructionScript)

(fn GetInteractableTooltipPosition
  (return (Transformation|GetWorldLocation (Variables|Default|GetTooltipPos))))

(fn SetMaterialonWheel
  (params (Material :type Material%20Interface%20Object%20Reference))
  (Rendering|Material|SetMaterial (Variables|Default|GetWheel) 0 Material)
  (Rendering|Material|SetMaterial (Variables|Default|GetHandle1) 0 Material)
  (Rendering|Material|SetMaterial (Variables|Default|GetHandle2) 0 Material)
  (Rendering|Material|SetMaterial (Variables|Default|GetHandle3) 0 Material)
  (Rendering|Material|SetMaterial (Variables|Default|GetHandle4) 0 Material)
  (Rendering|Material|SetMaterial (Variables|Default|GetHandle5) 0 Material)
  (Rendering|Material|SetMaterial (Variables|Default|GetHandle6) 0 Material)
  (Rendering|Material|SetMaterial (Variables|Default|GetHandle7) 0 Material)
  (Rendering|Material|SetMaterial (Variables|Default|GetHandle8) 0 Material))