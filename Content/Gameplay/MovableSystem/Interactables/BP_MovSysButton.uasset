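; BP_MovSysButton is an interactable button in the movable system that plays a press animation when its interact feedback event fires.
; The event resets a timer and enables Tick, which lerps the button mesh between pressed and base world positions using a curve over the press time.
; Tick disables itself when the timer completes.
; A TooltipPos component supplies the interaction tooltip location.
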(event EventTick
  (params (DeltaSeconds :type Float%20%28single-precision%29))
  (if (Variables|Default|GetbPressed)
    (Utilities|FlowControl|Sequence
      (:then_0
        (bind _output_get (Variables|ButtonFeedback|SetButtonPressTimer (+ (Variables|ButtonFeedback|GetButtonPressTimer) DeltaSeconds)))
        (if (>= _output_get (Variables|ButtonFeedback|GetButtonPressTime))
          (Variables|ButtonFeedback|SetButtonPressTimer (Variables|ButtonFeedback|GetButtonPressTime))
          (Variables|Default|SetbPressed false)
          (Actor|Tick|SetActorTickEnabled false)))
      (:then_1
        (Transformation|SetWorldLocation (Variables|Default|GetButton) (Math|Vector|Lerp(Vector) (Transformation|GetWorldLocation (Variables|Default|GetButtonPressedPos)) (Variables|ButtonFeedback|GetButtonPressBasePos) (Math|Curves|GetFloatValue (Variables|ButtonFeedback|GetButtonPressCurve) (/ (Variables|ButtonFeedback|GetButtonPressTimer) (Variables|ButtonFeedback|GetButtonPressTime)))) false false)))))

(event EventButtonInteractFeedback
  (Variables|Default|SetbPressed true)
  (Variables|ButtonFeedback|SetButtonPressTimer 0.0)
  (Actor|Tick|SetActorTickEnabled true))

(event EventBeginPlay
  (Variables|ButtonFeedback|SetButtonPressBasePos (Transformation|GetWorldLocation (Variables|Default|GetButton))))

(fn ConstructionScript)

(fn GetInteractableTooltipPosition
  (return (Transformation|GetWorldLocation (Variables|Default|GetTooltipPos))))