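; Main menu actor with clickable 3D mesh buttons for Play, Acts, Options and Exit, hiding the player pawn.
; Mouse events and InputNav set a shared button index, recolor child text renders for feedback, and clicks dispatch that index's action.
; Play opens the first level and Exit quits.
; Acts and Options blend to their own cameras, with a curve-driven timeline raising the actor or the HUD showing options; BacktoMenu restores the main view.
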(event Custom|OnBeginCursorOver_Event
  (params (TouchedComponent :type Primitive%20Component%20Object%20Reference))
  ;[0 1 0 0.33] OnBeginCursorOver_Event
  (bind _asstatic_mesh_component (Utilities|Casting|CastToStaticMeshComponent TouchedComponent))
  (Variables|Nav|SetIndexButtons (Utilities|Array|FindItem (Variables|Nav|GetButtons) _asstatic_mesh_component))
  (bind _astext_render_component (Utilities|Casting|CastToTextRenderComponent (Components|GetChildComponent _asstatic_mesh_component 0)))
  (CallFunction|AnimationsStartOver _astext_render_component))

(event Custom|OnEndCursorOver_Event
  (params (TouchedComponent :type Primitive%20Component%20Object%20Reference))
  ;[1 0 0 0.33] OnEndCursorOver_Event
  (bind _asstatic_mesh_component (Utilities|Casting|CastToStaticMeshComponent TouchedComponent))
  (Variables|Nav|SetIndexButtons (Utilities|Array|FindItem (Variables|Nav|GetButtons) _asstatic_mesh_component))
  (bind _astext_render_component (Utilities|Casting|CastToTextRenderComponent (Components|GetChildComponent _asstatic_mesh_component 0)))
  (CallFunction|AnimationsEndOver _astext_render_component))

(event Custom|OnClicked_Event
  (params (TouchedComponent :type Primitive%20Component%20Object%20Reference) (ButtonPressed :type Key%20Structure :default "None"))
  ;[1 1 0 0.33] OnClicked_Event
  (bind _asstatic_mesh_component (Utilities|Casting|CastToStaticMeshComponent TouchedComponent))
  (bind _astext_render_component (Utilities|Casting|CastToTextRenderComponent (Components|GetChildComponent _asstatic_mesh_component 0)))
  (Rendering|Components|TextRender|SetTextRenderColor _astext_render_component (Math|Color|MakeColor 0 100 100))
  (CallFunction|ButtonsActions)
  (Utilities|FlowControl|Delay 0.15)
  (Rendering|Components|TextRender|SetTextRenderColor _astext_render_component (Math|Color|MakeColor 0 0 100)))

(event Custom|AnimationsActs
  (params (isDown :type Boolean))
  (bind _initposition (Variables|Default|GetInitPosition))
  (if isDown
    (Game|Player|SetViewTargetwithBlend (Game|GetPlayerController 0) (Variables|ActionActs|GetCameraActs) (Variables|ActionActs|GetTimeCameraTravelActs) "VTBlend_Linear" 0.0 false)
    (bind _newtrack_0 (Timeline|T_AnimationActs PlayFromStart)
      (:Update
        (Transformation|SetActorLocation (Math|Vector|MakeVector (.x _initposition) (.y _initposition) (Math|Float|Lerp (.z _initposition) (+ (.z _initposition) (Variables|ActionActs|GetButtonsUpDistance)) (Math|Curves|GetFloatValue (Variables|ActionActs|GetCurveAnimationMenu) _newtrack_0))) false false)))
    (else
      (Game|Player|SetViewTargetwithBlend (Game|GetPlayerController 0) (Variables|Default|GetCamera) (Variables|ActionActs|GetTimeCameraTravelActs) "VTBlend_Linear" 0.0 false)
      (Timeline|T_AnimationActs ReverseFromEnd))))

(event EventInputNav
  (params (InputValue :type Float%20%28double-precision%29))
  ;[1 1 1] Navigation
  (if (< InputValue 0.0)
    (if (== (- (Variables|Nav|GetIndexButtons) 1) -1)
      _
      (else
        (Math|Integer|DecrementInt (Variables|Nav|GetIndexButtons)
          (:%20%20
            _))))
    (CallFunction|UpdateNavButton :!label _label)
    (elif (> InputValue 0.0)
      (if (== (Utilities|Array|Length (Variables|Nav|GetButtons)) (+ (Variables|Nav|GetIndexButtons) 1))
        (goto _label)
        (else
          (Math|Integer|IncrementInt (Variables|Nav|GetIndexButtons)
            (:%20%20
              (goto _label))))))))

(event EventButtonsActions
  (bind _returnvalue (Game|GetPlayerController 0))
  (bind _returnvalue_2 (Game|GetPlayerController 0))
  ;[0.5 1 0 0.33] Buttons Actions
  (switch int (Variables|Nav|GetIndexButtons)
    (:0
      ;;[1 1 1] Action Play
      (Variables|/Script/Engine.PlayerController|SetbShowMouseCursor (Game|GetPlayerController 0) false)
      (Game|OpenLevel(byObjectReference) (Variables|ActionPlay|GetFirstGameplayLvl)))
    (:1
      ;;[1 1 1] Action Acts
      (Development|PrintString "Action Acts")
      (CallFunction|AnimationsActs true))
    (:2
      ;;[1 1 1] Action Options
      (Variables|/Script/Engine.PlayerController|SetbShowMouseCursor _returnvalue_2 false)
      (Variables|/Script/Engine.PlayerController|SetbEnableMouseOverEvents _returnvalue_2 false)
      (Variables|/Script/Engine.PlayerController|SetbEnableClickEvents _returnvalue_2 false)
      (Game|Player|SetViewTargetwithBlend _returnvalue_2 (Variables|ActionOption|GetCameraOptions) (Variables|ActionOption|GetTimeCameraTravelOptions) "VTBlend_Linear" 0.0 false)
      (Utilities|FlowControl|Delay (Variables|ActionOption|GetTimeCameraTravelOptions))
      (Input|SetInputModeGameandUI _returnvalue 0 "LockOnCapture" false false)
      (Variables|/Script/Engine.PlayerController|SetbShowMouseCursor _returnvalue true)
      (Class|BPIHUDMenu|HiddeOptionMenu(Message) (HUD|GetHUD _returnvalue) false))
    (:3
      ;;[1 1 1] Action Exit
      (Game|QuitGame 0 "Quit" false))))

(event EventBeginPlay
  (bind _returnvalue (Game|GetPlayerController 0))
  (bind _buttons (Variables|Nav|GetButtons))
  (Rendering|SetActorHiddenInGame (Game|Player|GetPlayerPawn 0) true)
  (CallFunction|InitButtonOrder)
  (Game|Player|SetViewTargetwithBlend _returnvalue (Variables|Default|GetCamera) 0.0 "VTBlend_Linear" 0.0 false)
  (Variables|/Script/Engine.PlayerController|SetbShowMouseCursor _returnvalue true)
  (Variables|/Script/Engine.PlayerController|SetbEnableMouseOverEvents _returnvalue true)
  (Variables|/Script/Engine.PlayerController|SetbEnableClickEvents _returnvalue true)
  (Variables|Default|SetInitPosition (Transformation|GetActorLocation))
  ;[1 1 1] Bind event for buttons
  (EventDispatchers|BindEventtoOnBeginCursorOver _buttons (delegate Custom|OnBeginCursorOver_Event))
  (EventDispatchers|AssignOnEndCursorOver _buttons (delegate Custom|OnEndCursorOver_Event))
  (EventDispatchers|AssignOnClicked _buttons (delegate Custom|OnClicked_Event)))

(event EventBacktoMenu
  (bind _returnvalue (Game|GetPlayerController 0))
  (bind _returnvalue_2 (Game|GetPlayerController 0))
  (bind _returnvalue_3 (Game|GetPlayerController 0))
  (bind _timecameratraveloptions (Variables|ActionOption|GetTimeCameraTravelOptions))
  ;[1 1 1] Back to Main menu
  (Development|PrintString "Hello")
  (Input|SetInputModeGameOnly _returnvalue false)
  (Class|BPIHUDMenu|HiddeOptionMenu(Message) (HUD|GetHUD _returnvalue) true)
  (Variables|/Script/Engine.PlayerController|SetbShowMouseCursor _returnvalue_3 false)
  (Game|Player|SetViewTargetwithBlend _returnvalue_3 (Variables|Default|GetCamera) _timecameratraveloptions "VTBlend_Linear" 0.0 false)
  (Utilities|FlowControl|Delay _timecameratraveloptions)
  (Variables|/Script/Engine.PlayerController|SetbShowMouseCursor _returnvalue_2 true)
  (Variables|/Script/Engine.PlayerController|SetbEnableMouseOverEvents _returnvalue_2 true)
  (Variables|/Script/Engine.PlayerController|SetbEnableClickEvents _returnvalue_2 true))

(fn ConstructionScript)

(fn AnimationsStartOver
  (params (Text :type Text%20Render%20Component%20Object%20Reference))
  (Rendering|Components|TextRender|SetTextRenderColor Text (Math|Color|MakeColor 0 100 0 100)))

(fn AnimationsEndOver
  (params (Text :type Text%20Render%20Component%20Object%20Reference))
  (Rendering|Components|TextRender|SetTextRenderColor Text (Math|Color|MakeColor 0 0 100 100)))

(fn InitButtonOrder
  (Utilities|Array|Add (Variables|Nav|GetButtons) (Variables|Default|GetButtonPlay))
  (Utilities|Array|Add (Variables|Nav|GetButtons) (Variables|Default|GetButtonActs))
  (Utilities|Array|Add (Variables|Nav|GetButtons) (Variables|Default|GetButtonOptions))
  (Utilities|Array|Add (Variables|Nav|GetButtons) (Variables|Default|GetButtonExit)))

(fn UpdateNavButton
  (for _array_element (Variables|Nav|GetButtons)
    (bind _astext_render_component (Utilities|Casting|CastToTextRenderComponent (Components|GetChildComponent _array_element 0)))
    (Rendering|Components|TextRender|SetTextRenderColor _astext_render_component (Math|Color|MakeColor 0 0 100 100)))
  (bind _astext_render_component_2 (Utilities|Casting|CastToTextRenderComponent (Components|GetChildComponent (Utilities|Array|Get(acopy) (Variables|Nav|GetButtons) (Variables|Nav|GetIndexButtons)) 0)))
  (Rendering|Components|TextRender|SetTextRenderColor _astext_render_component_2 (Math|Color|MakeColor 0 100 0 100)))