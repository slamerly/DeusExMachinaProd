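; BP_ActsMenu is a 3D menu of act buttons, built from the unique values in the game instance's ScenesList.
; CreateButtons spawns stacked static meshes with text labels, which recolor on hover, click or InputNav navigation.
; A click calls AnimDisplayScenes, which starts a curve-driven timeline from a loop over unselected buttons to shift them along X.
; Scene sub-button creation and two vertical animations are present but never run.
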(event Custom|AnimDisplayScenes
  (params (Display :type Boolean) (IndexButtonSelected :type Integer))
  (for (_array_element _array_index) (Variables|Nav|GetButtonsActs)
    (if (!= IndexButtonSelected _array_index)
      (Development|PrintText (Utilities|Text|FormatText "entre:{indexentre} != {index}" IndexButtonSelected _array_index))
      (bind _newtrack_0 (Timeline|Timeline PlayFromStart)
        (:Update
          (Transformation|SetRelativeLocation _array_element (Math|Vector|MakeVector (Math|Float|Lerp (.x (Utilities|Array|Get(acopy) (Variables|Buttons|GetInitPositionButtonsAct) _array_index)) (+ (.x (Utilities|Array|Get(acopy) (Variables|Buttons|GetInitPositionButtonsAct) _array_index)) (Variables|ActionActs|GetButtonsBackDistance)) (Math|Curves|GetFloatValue (Variables|ActionActs|GetCurveAnimationButton) _newtrack_0)) (.y (Utilities|Array|Get(acopy) (Variables|Buttons|GetInitPositionButtonsAct) _array_index)) (.z (Utilities|Array|Get(acopy) (Variables|Buttons|GetInitPositionButtonsAct) _array_index))) false false))))))

(event Custom|OnBeginCursorOver_Event
  (params (TouchedComponent :type Primitive%20Component%20Object%20Reference))
  ;[0 1 0 0.33] OnBeginCursorOver_Event
  (bind _asstatic_mesh_component (Utilities|Casting|CastToStaticMeshComponent TouchedComponent))
  (Variables|Nav|SetIndexButtonsActs (Utilities|Array|FindItem (Variables|Nav|GetButtonsActs) _asstatic_mesh_component))
  (bind _astext_render_component (Utilities|Casting|CastToTextRenderComponent (Components|GetChildComponent _asstatic_mesh_component 0)))
  (CallFunction|AnimationsStartOver _astext_render_component))

(event Custom|OnEndCursorOver_Event
  (params (TouchedComponent :type Primitive%20Component%20Object%20Reference))
  ;[1 0 0 0.33] OnEndCursorOver_Event
  (bind _asstatic_mesh_component (Utilities|Casting|CastToStaticMeshComponent TouchedComponent))
  (Variables|Nav|SetIndexButtonsActs (Utilities|Array|FindItem (Variables|Nav|GetButtonsActs) _asstatic_mesh_component))
  (bind _astext_render_component (Utilities|Casting|CastToTextRenderComponent (Components|GetChildComponent _asstatic_mesh_component 0)))
  (CallFunction|AnimationsEndOver _astext_render_component))

(event Custom|OnClicked_Event
  (params (TouchedComponent :type Primitive%20Component%20Object%20Reference) (ButtonPressed :type Key%20Structure :default "None"))
  ;[1 1 0 0.33] OnClicked_Event
  (bind _asstatic_mesh_component (Utilities|Casting|CastToStaticMeshComponent TouchedComponent))
  (bind _astext_render_component (Utilities|Casting|CastToTextRenderComponent (Components|GetChildComponent _asstatic_mesh_component 0)))
  (Rendering|Components|TextRender|SetTextRenderColor _astext_render_component (Math|Color|MakeColor 0 100 100))
  (CallFunction|ButtonsActions)
  (Utilities|FlowControl|Delay 0.15)
  (Rendering|Components|TextRender|SetTextRenderColor _astext_render_component (Math|Color|MakeColor 0 0 100)))

(event EventInputNav
  (params (InputValue :type Float%20%28double-precision%29))
  ;[1 1 1] Navigation
  (if (< InputValue 0.0)
    (if (== (- (Variables|Nav|GetIndexButtonsActs) 1) -1)
      _
      (else
        (Math|Integer|DecrementInt (Variables|Nav|GetIndexButtonsActs)
          (:%20%20
            _))))
    (CallFunction|UpdateNavButton :!label _label)
    (elif (> InputValue 0.0)
      (if (== (Utilities|Array|Length (Variables|Nav|GetButtonsActs)) (+ (Variables|Nav|GetIndexButtonsActs) 1))
        (goto _label)
        (else
          (Math|Integer|IncrementInt (Variables|Nav|GetIndexButtonsActs)
            (:%20%20
              (goto _label))))))))

(event EventButtonsActions
  ;[0.5 1 0 0.33] Buttons Actions
  (CallFunction|AnimDisplayScenes false (Variables|Nav|GetIndexButtonsActs)))

(event EventBeginPlay
  (bind _buttonsacts (Variables|Nav|GetButtonsActs))
  (CallFunction|CreateButtons)
  ;[1 1 1] Bind event for buttons
  (EventDispatchers|BindEventtoOnBeginCursorOver _buttonsacts (delegate Custom|OnBeginCursorOver_Event))
  (EventDispatchers|AssignOnEndCursorOver _buttonsacts (delegate Custom|OnEndCursorOver_Event))
  (EventDispatchers|AssignOnClicked _buttonsacts (delegate Custom|OnClicked_Event)))

(fn ConstructionScript)

(fn AnimationsStartOver
  (params (Text :type Text%20Render%20Component%20Object%20Reference))
  (Rendering|Components|TextRender|SetTextRenderColor Text (Math|Color|MakeColor 0 100 0 100)))

(fn AnimationsEndOver
  (params (Text :type Text%20Render%20Component%20Object%20Reference))
  (Rendering|Components|TextRender|SetTextRenderColor Text (Math|Color|MakeColor 0 0 100 100)))

(fn UpdateNavButton
  (for _array_element (Variables|Nav|GetButtonsActs)
    (bind _astext_render_component (Utilities|Casting|CastToTextRenderComponent (Components|GetChildComponent _array_element 0)))
    (Rendering|Components|TextRender|SetTextRenderColor _astext_render_component (Math|Color|MakeColor 0 0 100 100)))
  (bind _astext_render_component_2 (Utilities|Casting|CastToTextRenderComponent (Components|GetChildComponent (Utilities|Array|Get(acopy) (Variables|Nav|GetButtonsActs) (Variables|Nav|GetIndexButtonsActs)) 0)))
  (Rendering|Components|TextRender|SetTextRenderColor _astext_render_component_2 (Math|Color|MakeColor 0 100 0 100)))

(fn CreateButtons
  (bind _asgame_instance_deus_ex (Utilities|Casting|CastToGameInstanceDeusEx (Game|GetGameInstance)))
  (bind _values (Utilities|Map|Values (Variables|/Script/DeusExMachina.GameInstanceDeusEx|GetScenesList _asgame_instance_deus_ex)))
  ;[1 1 1] Catch the different acts
  (for _array_element _values
    (Utilities|Array|AddUnique (LocalVariables|GetActsNames) _array_element))
  ;[1 1 1] Create the button for the act
  (for (_array_element_2 _array_index) (LocalVariables|GetActsNames)
    (Utilities|Array|Add (Variables|Buttons|GetInitPositionButtonsAct) (Math|Vector|MakeVector 0.0 0.0 (- (- 0.0 25.0) (* _array_index (Variables|Buttons|GetSpaceBetweenButtons)))))
    (bind _returnvalue (AddComponent|AddStaticMeshComponent false (Math|Transform|MakeTransform (Math|Vector|MakeVector 0.0 0.0 (- (- 0.0 25.0) (* _array_index (Variables|Buttons|GetSpaceBetweenButtons)))) "0, 0, 0" (Variables|Buttons|GetScaleStaticMesh))))
    (Utilities|Array|Add (Variables|Nav|GetButtonsActs) _returnvalue)
    (Utilities|Array|Add (Variables|Buttons|GetIndexesActs) 0)
    (bind _returnvalue_2 (AddComponent|AddTextRenderComponent false (Math|Transform|MakeTransform "-60.000000,0.000000,0.000000" "0.000000,180.000000,0.000000" "1.000000,0.400000,1.250000")))
    (Rendering|Components|TextRender|SetText _returnvalue_2 (Utilities|Text|ToText(Name) _array_element_2))
    (Rendering|Components|TextRender|SetHorizontalAlignment _returnvalue_2 "EHTA_Center")
    (Class|TextRenderComponent|SetVerticalAlignment _returnvalue_2 "EVRTA_TextCenter")
    (Rendering|Components|TextRender|SetTextRenderColor _returnvalue_2 (Math|Color|MakeColor 0 0 100 100))
    (Transformation|AttachComponentToComponent _returnvalue_2 _returnvalue "None" "KeepRelative" "KeepRelative" "KeepRelative" true)))