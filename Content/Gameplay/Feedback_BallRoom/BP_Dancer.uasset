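; BP_Dancer is a ballroom feedback actor whose arrow shows when it has turned roughly halfway around from its starting facing.
; It stores its rotation at BeginPlay, then each Tick compares the current yaw against that start.
; The arrow turns green while the yaw difference is near 180 degrees in either direction and red otherwise.
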(event EventBeginPlay
  (Variables|Default|SetStartRotator (Transformation|GetActorRotation)))

(event Collision|EventActorBeginOverlap
  (params (OtherActor :type Actor%20Object%20Reference)))

(event EventTick
  (params (DeltaSeconds :type Float%20%28single-precision%29))
  (bind _arrow (Variables|Default|GetArrow))
  ;[0.553 1 0] Arrow Become green
  (if (> (Math|Float|Absolute(Float) (.yaw (Math|Rotator|Delta(Rotator) (Variables|Default|GetStartRotator) (Transformation|GetActorRotation)))) 1.7e+02)
    (Components|Arrow|SetArrowColor(LinearColor) _arrow "(R=0.259547,G=1.000000,B=0.000000,A=1.000000)")
    (else
      (Components|Arrow|SetArrowColor(LinearColor) _arrow "(R=1.000000,G=0.020031,B=0.000000,A=1.000000)"))))

(fn ConstructionScript)