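; Hovering spotlight eye that watches for the player and reloads the level once it sees them.
; Targeting holds its rotation, follows the player within a clamped angle, or ping-pongs between target points, with Perlin-noise wiggle and hover.
; Detection uses cached per-tick vectors for range and cone checks before a line-of-sight trace.
; Random timers drive a timeline blink that rotates both lids and scales the light, with occasional double blinks.
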(event Custom|SwitchToNextPosition
  (switch int (Variables|Behaviour|FixedPositions|GetCurrentDirection)
    (:-1
      ;[0.1772 0.1363 0.3125] Are we at the extremes?
      (if (== (Variables|Behaviour|FixedPositions|GetCurrentFixedPositionIndex) 0)
        (CallFunction|MultiplyValueInt (Variables|Behaviour|FixedPositions|GetCurrentDirection) -1 :!label _label)
        (CallFunction|SwitchtoNextPosition)
        (else
          (CallFunction|IncreaseValueInt (Variables|Behaviour|FixedPositions|GetCurrentFixedPositionIndex) (Variables|Behaviour|FixedPositions|GetCurrentDirection) :!label _label_2)
          (Variables|Behaviour|FixedPositions|SetFixedPositionCanMove true))))
    (:1
      (if (== (Variables|Behaviour|FixedPositions|GetCurrentFixedPositionIndex) (Utilities|Array|LastIndex (Variables|Behaviour|FixedPositions|GetFixedPositionsArray)))
        (goto _label)
        (else
          (goto _label_2))))))

(event Custom|Blink
  ;[1 1 1] For quickness' sake, the first blink of a double-blink should be faster.
  ; In-game it feels like both are the same length, so it's good like that because otherwise it's too slow
  (if (== (Variables|Default|GetCurrentBlink) (Variables|Default|GetNextDoubleBlink))
    (Components|Timeline|SetPlayRate (Variables|Default|GetBlinkTimeline) 1.5)
    (bind _eyerotation (Timeline|BlinkTimeline PlayFromStart)
      (:Update
        (Transformation|SetRelativeRotation (Variables|Default|GetTopBit) (Math|Rotator|MakeRotator 0.0 _eyerotation 0.0) false false)
        (Transformation|SetRelativeRotation (Variables|Default|GetBottomBit) (Math|Rotator|MakeRotator 0.0 (* _eyerotation -1.0) 0.0) false false)
        (Rendering|Components|Light|SetIntensity (Variables|Default|GetSpotLight) (* (/ (+ _eyerotation 6e+01) 9e+01) (Variables|LightSettings|GetLightIntensityCandela))))
      (:Finished
        (if (== (Variables|Default|GetCurrentBlink) (Variables|Default|GetNextDoubleBlink))
          (CallFunction|NewDoubleBlink)
          (CallFunction|Blink)
          (else
            (Blinks|StartNewBlink)))))
    (else
      (Components|Timeline|SetPlayRate (Variables|Default|GetBlinkTimeline) 1.0)
      (Timeline|BlinkTimeline PlayFromStart))))

(event EventBeginPlay
  (References|GetReferences)
  (Variables|Behaviour|PlayerResponse|SetHasSeenPlayer false)
  (CallFunction|NewDoubleBlink)
  (Blinks|StartNewBlink)
  (if (Utilities|Enum|Equal(Enum) (Variables|Behaviour|GetTargeting%20Mode) "NewEnumerator2")
    (Variables|Behaviour|FixedPositions|SetCurrentFixedPositionIndex 0)
    (Variables|Behaviour|FixedPositions|SetCurrentDirection 1)
    (bind _returnvalue (Utilities|Time|SetTimerbyEvent (EventDispatchers|CreateEvent :!event Custom|SwitchToNextPosition) (Variables|Behaviour|FixedPositions|GetTimeSpentAtEachPosition) true))
    (Variables|Behaviour|FixedPositions|SetFixedPositionSwitchTimerHandle _returnvalue)))

(event EventTick
  (params (DeltaSeconds :type Float%20%28single-precision%29))
  (CachedData|CacheTickValues)
  (Utilities|FlowControl|Sequence
    (:then_0
      (Behaviour|FollowTargetingBehaviour))
    (:then_1
      (if (Variables|Behaviour|GetShouldDetectPlayer)
        (Behaviour|TrytoDetectPlayer)))
    (:then_2
      ;[0 0 0] I know that you should NOT have multiple Transform updates per actor, you should cache the final Location and Rotation and then do only ONE SetActorLocationAndRotation
      ; If this needs optimization this can be done; for now it's not an issue.
      (if (Variables|Hover|GetShouldHover)
        (Hover|ApplyCustomHover)))
    (:then_3
      ;[1 0 0] DEBUG
      (if (Variables|Debug|GetShouldDebug)
        (Development|PrintText (Utilities|Text|FormatText "Next Blink in {s} seconds 
Double blink in {n} blinks" (Utilities|Time|GetTimerRemainingTimebyHandle (Variables|Blinks|GetNextBlinkTimerHandle)) (- (Variables|Default|GetNextDoubleBlink) (Variables|Default|GetCurrentBlink))) true true "(R=1.000000,G=0.638744,B=0.295815,A=1.000000)" 2.0 (Utilities|String|StringToName (Utilities|GetDisplayName self)))))))

(fn ConstructionScript
  (Rendering|Lighting|SetAttenuationRadius (Variables|Default|GetSpotLight) (Variables|LightSettings|GetLightAttenuationRadius))
  (Rendering|Components|Light|SetIntensity (Variables|Default|GetSpotLight) (Variables|LightSettings|GetLightIntensityCandela))
  (Rendering|Lighting|SetInnerConeAngle (Variables|Default|GetSpotLight) (Variables|LightSettings|GetLightInnerConeAngle))
  (Rendering|Lighting|SetOuterConeAngle (Variables|Default|GetSpotLight) (Variables|LightSettings|GetLightOuterConeAngle))
  (Class|LightComponent|SetTemperature (Variables|Default|GetSpotLight) (Variables|LightSettings|GetLightTemperature))
  (Class|LightComponent|SetVolumetricScatteringIntensity (Variables|Default|GetSpotLight) (Variables|LightSettings|GetLightVolumetricScatteringIntensity))
  (Class|PointLightComponent|SetSourceRadius (Variables|Default|GetSpotLight) (Variables|LightSettings|GetLightSourceRadius))
  (Class|PointLightComponent|SetSoftSourceRadius (Variables|Default|GetSpotLight) (Variables|LightSettings|GetLightSoftSourceRadius)))

(fn GetReferences
  (Utilities|FlowControl|Sequence
    (:then_0
      (bind _output_get (Variables|References|SetPlayerReference (Game|Player|GetPlayerPawn 0)))
      (Utilities|IsValid _output_get
        (:Is%20Not%20Valid
          (Development|PrintString "BP_ProjectorEye couldn't find the Player!!" true true "(R=1.000000,G=0.000000,B=0.000000,A=1.000000)" 5e+01))))
    (:then_1
      (Variables|CachedData|SetStartingForward (Transformation|GetActorForwardVector))
      (Variables|CachedData|SetStartingRotation (Transformation|GetActorRotation))
      (Variables|CachedData|SetCachedStartingLocation (Transformation|GetActorLocation)))))

(fn FollowTargetingBehaviour
  (switch Utilities|FlowControl|Switch|SwitchonE_EyeTargetMode (Variables|Behaviour|GetTargeting%20Mode)
    (:NewEnumerator0
      (if (Variables|Wiggle|GetShouldWiggle)
        (bind (_addedpitch _addedyaw) (Wiggle|ComputeCustomWiggle))
        (Transformation|SetActorRotation (Math|Rotator|CombineRotators (Variables|CachedData|GetStartingRotation) (Math|Rotator|MakeRotator 0.0 _addedpitch _addedyaw)))))
    (:NewEnumerator1
      (Behaviour|FollowPlayer|UpdateFollowPlayerTargeting))
    (:NewEnumerator2
      (Behaviour|FixedPositions|UpdateFixedPositionTargeting))))

(fn DebugLinestoPlayer
  (bind _cachedeyelocation (Variables|CachedData|GetCachedEyeLocation))
  (Rendering|Debug|FlushPersistentDebugLines)
  (Rendering|Debug|DrawDebugLine (Variables|CachedData|GetCachedEyeLocation) (Variables|CachedData|GetCachedPlayerLocation) "(R=1.000000,G=0.000000,B=0.000000,A=1.000000)" 1e+01 2.0)
  (Rendering|Debug|DrawDebugLine _cachedeyelocation (+ _cachedeyelocation (* (Transformation|GetActorForwardVector) 5e+02)) "(R=0.000000,G=0.864498,B=1.000000,A=1.000000)" 1e+01 2.0)
  (Development|PrintString (Utilities|String|ToString(Float) (Class|KismetMathLibrary|DegAcos (Math|Vector|DotProduct (Transformation|GetActorForwardVector) (Math|Vector|Normalize (Variables|CachedData|GetVectorToPlayer))))) true true "(R=0.000000,G=0.660000,B=1.000000,A=1.000000)" 2.0 "237275"))

(fn CacheTickValues
  (Utilities|FlowControl|Sequence
    (:then_0
      ;[0.3177 0.1076 0.2882] Eye-Player location data
      (Variables|CachedData|SetCachedPlayerLocation (Transformation|GetActorLocation (Variables|References|GetPlayerReference)))
      (Variables|CachedData|SetCachedEyeLocation (Transformation|GetActorLocation))
      (Variables|CachedData|SetVectorToPlayer (- (Variables|CachedData|GetCachedPlayerLocation) (Variables|CachedData|GetCachedEyeLocation)))
      (Variables|CachedData|SetCachedAngleToPlayer (Class|KismetMathLibrary|DegAcos (Math|Vector|DotProduct (Transformation|GetActorForwardVector) (Math|Vector|Normalize (Variables|CachedData|GetVectorToPlayer))))))
    (:then_1
      ;[0.1021 0.276 0.1272] Other Data
      (Variables|CachedData|SetCachedCurrentActorTime (Actor|GetGameTimeSinceCreation)))))

(fn DebugConeDetection
  (bind _maxplayerconedetectionangle (Variables|Behaviour|GetMaxPlayerConeDetectionAngle))
  (Rendering|Debug|FlushPersistentDebugLines)
  (Class|KismetSystemLibrary|DrawDebugConeinDegrees (Transformation|GetActorLocation) (Transformation|GetActorForwardVector) (Variables|Behaviour|GetMaxPlayerConeDetectionRange) _maxplayerconedetectionangle _maxplayerconedetectionangle 16 "(R=1.000000,G=0.099000,B=0.000000,A=1.000000)" 1e+01 0.0))

(fn SeeingthePlayer
  ;[0 0 0] Probably an Event Dispatcher Hub call to make all changes without references (fade to black, stop inputs, play a sound, maybe the environment will react...)
  (if (not (Variables|Behaviour|PlayerResponse|GetHasSeenPlayer))
    (Variables|Behaviour|PlayerResponse|SetHasSeenPlayer true)
    (bind _returnvalue (Game|GetCurrentLevelName true))
    (Game|OpenLevel(byName) (Utilities|String|StringToName _returnvalue))))

(fn LineOfSightIsBlocked)

(fn PlayerIsOutsideAngle)

(fn TrytoDetectPlayer
  ;[0.3068 0.1462 0.401] Is the player close enough?
  (if (<= (Math|Vector|Distance(Vector) (Variables|CachedData|GetCachedPlayerLocation) (Variables|CachedData|GetCachedEyeLocation)) (Variables|Behaviour|GetMaxPlayerConeDetectionRange))
    ;[0.05847 0.2292 0.09308] Verify if the player is in the right angle before doing any LOS check
    ; This is more or less redundant for FollowPlayer Targeting Mode, but it's just an If statement...
    (if (>= (Variables|Behaviour|GetMaxPlayerConeDetectionAngle) (Variables|CachedData|GetCachedAngleToPlayer))
      (bind (_outhit _returnvalue) (Collision|LineTraceByChannel (Variables|CachedData|GetCachedEyeLocation) (Variables|CachedData|GetCachedPlayerLocation) "TraceTypeQuery2" false 0 "None"))
      (if _returnvalue
        ;[0.2865 0.06117 0.2736] We hit something!
        ; Is it the player or not?
        (if (== (Variables|References|GetPlayerReference) (.HitActor (Collision|BreakHitResult _outhit)))
          ;[1 0 0] DEBUG
          (if (Variables|Debug|GetShouldDebug)
            (Development|PrintText (Utilities|Text|FormatText "Eye Projector {name} sees Player" (Utilities|GetDisplayName self)) true true "(R=0.950000,G=0.000000,B=1.000000,A=1.000000)" 0.1))
          (Behaviour|PlayerResponse|SeeingthePlayer)
          (else
            (if (Variables|Debug|GetShouldDebug)
              (Development|PrintText (Utilities|Text|FormatText "Eye Projector {name} doesn't see the Player because there's something blocking the way" (Utilities|GetDisplayName self)) true true "(R=0.065411,G=0.000000,B=1.000000,A=1.000000)" 0.1))
            (Behaviour|PlayerResponse|LineOfSightIsBlocked)))
        (else
          ;[0 0 0] This is weird... The player should be hit by the Line Trace...
          (Development|PrintString "Nothing was hit by the Eye's Line Trace... 
Normally the Player should be hit if there is nothing blocking the ray. 
Something is probably wrong" true true "(R=1.000000,G=1.000000,B=0.000000,A=1.000000)" 2.0 "WeirdEyeProjectorRaycast")))
      (else
        (Behaviour|PlayerResponse|PlayerIsOutsideAngle)
        ;[1 0 0] DEBUG
        (if (Variables|Debug|GetShouldDebug)
          (Development|PrintText (Utilities|Text|FormatText "Eye Projector {name} doesn't see the Player because of the angle" (Utilities|GetDisplayName self)) true true "(R=0.227000,G=0.000000,B=1.000000,A=1.000000)" 0.1))))
    (else
      (Behaviour|PlayerResponse|PlayerIsTooFarAway)
      ;[1 0 0] DEBUG
      (if (Variables|Debug|GetShouldDebug)
        (Development|PrintText (Utilities|Text|FormatText "Eye Projector {name} doesn't see the Player because it is too far away" (Utilities|GetDisplayName self)) true true "(R=0.000000,G=0.428203,B=1.000000,A=1.000000)" 0.1)))))

(fn DebugFollowPlayerModeCone
  (bind _followplayermaxangle (Variables|Behaviour|FollowPlayer|GetFollowPlayerMaxAngle))
  (bind _startingforward (Variables|CachedData|GetStartingForward))
  (Rendering|Debug|FlushPersistentDebugLines)
  (Class|KismetSystemLibrary|DrawDebugConeinDegrees (Transformation|GetActorLocation) (Math|Vector|SelectVector (Transformation|GetActorForwardVector) _startingforward (Math|Vector|VectorIsZero _startingforward)) (Variables|Behaviour|GetMaxPlayerConeDetectionRange) _followplayermaxangle _followplayermaxangle 16 "(R=1.000000,G=0.000000,B=0.500000,A=1.000000)" 1e+01 0.0))

(fn SpawnNewTargetPoint
  (bind _returnvalue (Game|SpawnActorfromClass "/Game/Gameplay/Eyes/BP_EyeTargetPoint.BP_EyeTargetPoint_C" (Math|Transform|MakeTransform (+ (Transformation|GetActorLocation) (* (Transformation|GetActorForwardVector) 3e+02)) "0, 0, 0" "1.000000,1.000000,1.000000") "Undefined" "MultiplyWithRoot" 0 0))
  (Utilities|Array|Add (Variables|Behaviour|FixedPositions|GetFixedPositionsArray) _returnvalue))

(fn PlayerIsTooFarAway)

(fn ApplyCustomHover
  (Transformation|SetActorLocation (+ (Variables|CachedData|GetCachedStartingLocation) (* (Transformation|GetActorRightVector) (* (Class|KismetMathLibrary|PerlinNoise1D (* (Variables|CachedData|GetCachedCurrentActorTime) (Variables|Hover|GetHorizontalHoverFrequency))) (Variables|Hover|GetHorizontalHoverIntensity))) (* (Transformation|GetActorUpVector) (* (Class|KismetMathLibrary|PerlinNoise1D (* (Variables|CachedData|GetCachedCurrentActorTime) (Variables|Hover|GetVerticalHoverFrequency))) (Variables|Hover|GetVerticalHoverIntensity)))) false false))

(fn ComputeCustomWiggle
  (return (* (Class|KismetMathLibrary|PerlinNoise1D (* (Variables|CachedData|GetCachedCurrentActorTime) (Variables|Wiggle|GetPitchWiggleFrequency))) (Variables|Wiggle|GetPitchWiggleIntensity)) (* (Class|KismetMathLibrary|PerlinNoise1D (* (Variables|CachedData|GetCachedCurrentActorTime) (Variables|Wiggle|GetYawWiggleFrequency))) (Variables|Wiggle|GetYawWiggleIntensity))))

(fn UpdateFixedPositionTargeting
  (if (Variables|Behaviour|FixedPositions|GetFixedPositionCanMove)
    ;[0.5781 0.1506 0.4301] Rotate step
    (if (Variables|Wiggle|GetShouldWiggle)
      (bind (_addedpitch _addedyaw) (Wiggle|ComputeCustomWiggle))
      (Transformation|SetActorRotation (Math|Interpolation|RInterpTo (Transformation|GetActorRotation) (Math|Rotator|CombineRotators (Math|Rotator|FindLookatRotation (Variables|CachedData|GetCachedEyeLocation) (Transformation|GetActorLocation (Utilities|Array|Get(acopy) (Variables|Behaviour|FixedPositions|GetFixedPositionsArray) (Variables|Behaviour|FixedPositions|GetCurrentFixedPositionIndex)))) (Math|Rotator|MakeRotator 0.0 _addedpitch _addedyaw)) (Utilities|Time|GetWorldDeltaSeconds) (Variables|Behaviour|FixedPositions|GetFixedPositionTargetRotationSpeed)))
      (else
        (Transformation|SetActorRotation (Math|Interpolation|RInterpTo (Transformation|GetActorRotation) (Math|Rotator|FindLookatRotation (Variables|CachedData|GetCachedEyeLocation) (Transformation|GetActorLocation (Utilities|Array|Get(acopy) (Variables|Behaviour|FixedPositions|GetFixedPositionsArray) (Variables|Behaviour|FixedPositions|GetCurrentFixedPositionIndex)))) (Utilities|Time|GetWorldDeltaSeconds) (Variables|Behaviour|FixedPositions|GetFixedPositionTargetRotationSpeed)))))
    ;[0.375 0.1614 0.09741] Check if we attained the target
    (if (< (Class|KismetMathLibrary|DegAcos (Math|Vector|DotProduct (Transformation|GetActorForwardVector) (Math|Vector|Normalize (- (Transformation|GetActorLocation (Utilities|Array|Get(acopy) (Variables|Behaviour|FixedPositions|GetFixedPositionsArray) (Variables|Behaviour|FixedPositions|GetCurrentFixedPositionIndex))) (Variables|CachedData|GetCachedEyeLocation))))) 0.1)
      (Variables|Behaviour|FixedPositions|SetFixedPositionCanMove false)
      (Variables|Behaviour|FixedPositions|SetFixedPositionGoodRotation (Transformation|GetActorRotation)))
    (elif (Variables|Wiggle|GetShouldWiggle)
      (bind (_addedpitch_2 _addedyaw_2) (Wiggle|ComputeCustomWiggle))
      (Transformation|SetActorRotation (Math|Rotator|CombineRotators (Variables|Behaviour|FixedPositions|GetFixedPositionGoodRotation) (Math|Rotator|MakeRotator 0.0 _addedpitch_2 _addedyaw_2))))))

(fn UpdateFollowPlayerTargeting
  (bind _cachedeyelocation (Variables|CachedData|GetCachedEyeLocation))
  (bind _cachedplayerlocation (Variables|CachedData|GetCachedPlayerLocation))
  (bind _returnvalue (Math|Rotator|FindLookatRotation _cachedeyelocation _cachedplayerlocation))
  ;[1 0 0] DEBUG
  (if (Variables|Debug|GetShouldDebug)
    (Debug|DebugFollowPlayerModeCone))
  ;[0.009302 0.04321 0.05208] For the FollowPlayer:
  ; Compare the angle between the Starting Rotation and the target "Look at the Player" rotation, and if the difference exceeds the FollowPlayerMaxAngle, it will stop turning
  (bind _output_get (LocalVariables|SetFollowPlayer_AngleStartAndFollow (Class|KismetMathLibrary|DegAcos (Math|Vector|DotProduct (Variables|CachedData|GetStartingForward) (Math|Vector|Normalize (Variables|CachedData|GetVectorToPlayer))))))
  ;;[1 1 1] Is the target rotation within the allowed Angle margin?
  (if (<= _output_get (Variables|Behaviour|FollowPlayer|GetFollowPlayerMaxAngle))
    (if (Variables|Wiggle|GetShouldWiggle)
      (bind (_addedpitch _addedyaw) (Wiggle|ComputeCustomWiggle))
      (Transformation|SetActorRotation (Math|Rotator|CombineRotators _returnvalue (Math|Rotator|MakeRotator 0.0 _addedpitch _addedyaw)))
      (else
        (Transformation|SetActorRotation _returnvalue)))
    (elif (Variables|Wiggle|GetShouldWiggle)
      (bind (_addedpitch_2 _addedyaw_2) (Wiggle|ComputeCustomWiggle))
      (Transformation|SetActorRotation (Math|Rotator|CombineRotators (Math|Rotator|Lerp(Rotator) (Variables|CachedData|GetStartingRotation) (Math|Rotator|FindLookatRotation (Variables|CachedData|GetCachedEyeLocation) (Variables|CachedData|GetCachedPlayerLocation)) (/ (Variables|Behaviour|FollowPlayer|GetFollowPlayerMaxAngle) (LocalVariables|GetFollowPlayer_AngleStartAndFollow)) true) (Math|Rotator|MakeRotator 0.0 _addedpitch_2 _addedyaw_2)))
      (else
        (Transformation|SetActorRotation (Math|Rotator|Lerp(Rotator) (Variables|CachedData|GetStartingRotation) (Math|Rotator|FindLookatRotation (Variables|CachedData|GetCachedEyeLocation) (Variables|CachedData|GetCachedPlayerLocation)) (/ (Variables|Behaviour|FollowPlayer|GetFollowPlayerMaxAngle) (LocalVariables|GetFollowPlayer_AngleStartAndFollow)) true))))))

(fn StartNewBlink
  (bind _time_between_blinks (Variables|Blinks|GetTime%20Between%20Blinks))
  (bind _returnvalue (Utilities|Time|SetTimerbyEvent (EventDispatchers|CreateEvent :!event Custom|Blink) (Math|Random|RandomFloatinRange (.x _time_between_blinks) (.y _time_between_blinks))))
  (Variables|Blinks|SetNextBlinkTimerHandle _returnvalue)
  (Math|Integer|IncrementInt (Variables|Default|GetCurrentBlink)))

(fn NewDoubleBlink
  (Variables|Default|SetNextDoubleBlink (Math|Random|RandomIntegerinRange 3 7))
  (Variables|Default|SetCurrentBlink 1))