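; BP_PlayerWalkableSpline is a spline actor that defines a path for the player character to follow.
; On BeginPlay it caches the player, then traces down at each spline point and moves hit points to capsule half-height above the ground.
; This lets the player take point locations directly without sinking or floating.
; If ShouldExist is set, it then passes itself to the player's FollowNewSpline.
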(event EventBeginPlay
  (Utilities|FlowControl|Sequence
    (:then_0
      (bind _asbpc_deux_ex_player_character (Utilities|Casting|CastToBPC_DeuxExPlayerCharacter (Game|Player|GetPlayerPawn 0))
        (:then
          (Variables|Default|SetPlayer%20Reference _asbpc_deux_ex_player_character))
        (:CastFailed
          (Development|PrintString "BP_PlayerWalkableSpline doesn't find the BPC_Player_CameraTest... 
Maybe the class of the Player has changed?" true true "(R=1.000000,G=0.000000,B=0.000000,A=1.000000)" 5e+01))))
    (:then_1
      (bind _output_get (Variables|Default|SetNumberOfPoints (Spline|GetNumberOfSplinePoints (Variables|Default|GetSpline))))
      ;[1 0.7663 0.4042] Loop through each point and place it above ground at exactly the half-height of the Player Character; so he can take the X Y Z location as is and not be teleported in the ground or in the air
      (for _index (range 0 (- _output_get 1))
        (bind (_outhit _returnvalue) (Collision|LineTraceByChannel (+ (Spline|GetLocationatSplinePoint (Variables|Default|GetSpline) _index "World") (Math|Vector|MakeVector 0.0 0.0 5e+01)) (- (Spline|GetLocationatSplinePoint (Variables|Default|GetSpline) _index "World") (Math|Vector|MakeVector 0.0 0.0 5e+02)) "TraceTypeQuery1" false 0 "None"))
        (if _returnvalue
          (Spline|SetLocationatSplinePoint (Variables|Default|GetSpline) _index (+ (.Location (Collision|BreakHitResult _outhit)) (Math|Vector|MakeVector 0.0 0.0 (Components|Capsule|GetScaledCapsuleHalfHeight (Variables|/Script/Engine.Character|GetCapsuleComponent (Variables|Default|GetPlayer%20Reference))))) "World" true))))
    (:then_2
      (if (Variables|Default|GetShouldExist)
        ;[1 0.3542 0.7771] Tell the player to follow it
        (Default|FollowNewSpline (Variables|Default|GetPlayer%20Reference) self)))))

(fn ConstructionScript)