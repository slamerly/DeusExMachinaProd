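; Spline actor that constrains player walking to a path, with the Player Controller doing the following since it handles input.
; On BeginPlay it caches the player character, then line-traces at each spline point to snap it to capsule half-height above the ground, making closest-point lookups more precise.
; If ShouldExist is set, it sends interface messages registering itself with the controller and enabling spline following.
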(event EventBeginPlay
  (bind _returnvalue (Game|GetPlayerController 0))
  (Utilities|FlowControl|Sequence
    (:then_0
      (bind _asbpc_deux_ex_player_character (Utilities|Casting|CastToBPC_DeuxExPlayerCharacter (Game|Player|GetPlayerPawn 0))
        (:then
          (Variables|Default|SetPlayer%20Reference _asbpc_deux_ex_player_character))
        (:CastFailed
          (Development|PrintString "BP_PlayerConstraintWalkableSpline doesn't find the BPC_DeusExPlayerCharacter... 
Maybe the class of the Player has changed?" true true "(R=1.000000,G=0.000000,B=0.000000,A=1.000000)" 5e+01))))
    (:then_1
      (bind _output_get (Variables|Default|SetNumberOfPoints (Spline|GetNumberOfSplinePoints (Variables|Default|GetSpline))))
      ;[1 0.7663 0.4042] Loop through each point and place it above ground at exactly the half-height of the Player Character, so the "Get Location Closest To Point" can be more precise
      (for _index (range 0 (- _output_get 1))
        (bind (_outhit _returnvalue_2) (Collision|LineTraceByChannel (+ (Spline|GetLocationatSplinePoint (Variables|Default|GetSpline) _index "World") (Math|Vector|MakeVector 0.0 0.0 5e+01)) (- (Spline|GetLocationatSplinePoint (Variables|Default|GetSpline) _index "World") (Math|Vector|MakeVector 0.0 0.0 5e+02)) "TraceTypeQuery1" false 0 "None"))
        (if _returnvalue_2
          (Spline|SetLocationatSplinePoint (Variables|Default|GetSpline) _index (+ (.Location (Collision|BreakHitResult _outhit)) (Math|Vector|MakeVector 0.0 0.0 (Components|Capsule|GetScaledCapsuleHalfHeight (Variables|/Script/Engine.Character|GetCapsuleComponent (Variables|Default|GetPlayer%20Reference))))) "World" true))))
    (:then_2
      (if (Variables|Default|GetShouldExist)
        ;[1 0.3542 0.7771] Tell the Controller to follow it (since the Controller handles inputs)
        (Class|BPIPlayerController|ChangeConstraintSplinetoFollow(Message) _returnvalue self)
        (Class|BPIPlayerController|SetShouldFollowConstraintSplineBoolean(Message) _returnvalue true)))))

(fn ConstructionScript)