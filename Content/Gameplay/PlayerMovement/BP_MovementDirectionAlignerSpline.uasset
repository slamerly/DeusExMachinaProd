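; Spline actor that supplies a movement direction for the player controller to follow.
; On BeginPlay it traces each spline point to the ground, raises it by the player capsule's half-height for precise closest-point queries, and registers with the controller if ShouldExist is set.
; Show Directions previews the forward and right axes with timed debug arrows and labels, derived from the first point's tangent and the SplineDirection setting.
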(event Custom|ConstructHideText
  (Rendering|SetVisibility (Variables|Default|GetForwardAxisText) false false))

(event EventBeginPlay
  (bind _returnvalue (Game|GetPlayerController 0))
  (Utilities|FlowControl|Sequence
    (:then_0
      (bind _asbpc_deux_ex_player_character (Utilities|Casting|CastToBPC_DeuxExPlayerCharacter (Game|Player|GetPlayerPawn 0))
        (:then
          (Variables|Default|SetPlayer%20Reference _asbpc_deux_ex_player_character))
        (:CastFailed
          (Development|PrintString "BP_PlayerWalkableSpline doesn't find the BPC_Player_CameraTest... 
Maybe the class of the Player has changed?" true true "(R=1.000000,G=0.000000,B=0.000000,A=1.000000)" 5e+01))))
    (:then_1
      (bind _output_get (Variables|Default|SetNumberOfPoints (Spline|GetNumberOfSplinePoints (Variables|Default|GetSpline))))
      ;[1 0.7663 0.4042] Loop through each point and place it above ground at exactly the half-height of the Player Character, so the "Get Location Closest To Point" can be more precise
      (for _index (range 0 (- _output_get 1))
        (bind (_outhit _returnvalue_2) (Collision|LineTraceByChannel (+ (Spline|GetLocationatSplinePoint (Variables|Default|GetSpline) _index "World") (Math|Vector|MakeVector 0.0 0.0 5e+01)) (- (Spline|GetLocationatSplinePoint (Variables|Default|GetSpline) _index "World") (Math|Vector|MakeVector 0.0 0.0 5e+02)) "TraceTypeQuery1" false 0 "None"))
        (if _returnvalue_2
          (Spline|SetLocationatSplinePoint (Variables|Default|GetSpline) _index (+ (.Location (Collision|BreakHitResult _outhit)) (Math|Vector|MakeVector 0.0 0.0 (Components|Capsule|GetScaledCapsuleHalfHeight (Variables|/Script/Engine.Character|GetCapsuleComponent (Variables|Default|GetPlayer%20Reference))))) "World" true))))
    (:then_2
      (if (Variables|Setup|GetShould%20Exist?)
        (Class|BPIPlayerController|ChangeDirectionSplinetoFollow(Message) _returnvalue self)
        (Class|BPIPlayerController|SetShouldFollowDirectionSplineBoolean(Message) _returnvalue true)))
    (:then_3
      (Components|DestroyComponent (Variables|Default|GetRightAxisText)))))

(fn ConstructionScript)

(fn ShowDirections
  (bind _spline (Variables|Default|GetSpline))
  (Rendering|Debug|FlushPersistentDebugLines)
  (LocalVariables|SetConstruct_StartingPoint (+ (Spline|GetLocationatSplinePoint _spline 0 "World") "0.000000,0.000000,150.000000"))
  (LocalVariables|SetConstruct_SplineDirection (Math|Vector|Normalize (Spline|GetTangentatSplinePoint _spline 0 "World")))
  (Rendering|SetVisibility (Variables|Default|GetForwardAxisText) true false)
  (Utilities|Time|SetTimerbyEvent (EventDispatchers|CreateEvent :!event Custom|ConstructHideText) 15.0)
  (switch Utilities|FlowControl|Switch|SwitchonEMovementDirectionSplineWay (Variables|Setup|GetSpline%20Direction)
    (:NewEnumerator0
      (LocalVariables|SetConstruct_LineEnd (+ (LocalVariables|GetConstruct_StartingPoint) (* (LocalVariables|GetConstruct_SplineDirection) (Math|Float|MakeLiteralFloat 1e+02))))
      (Rendering|Debug|DrawDebugArrow (LocalVariables|GetConstruct_StartingPoint) (LocalVariables|GetConstruct_LineEnd) 5e+01 "(R=0.000000,G=1.000000,B=0.000000,A=1.000000)" 15.0 2.0)
      (Transformation|SetWorldLocation (Variables|Default|GetRightAxisText) (LocalVariables|GetConstruct_LineEnd) false false)
      (LocalVariables|SetConstruct_LineEnd (+ (LocalVariables|GetConstruct_StartingPoint) (* (Math|Vector|RotateVectorAroundAxis (LocalVariables|GetConstruct_SplineDirection) -9e+01 "0.000000,0.000000,1.000000") (Math|Float|MakeLiteralFloat 1e+02))))
      (Rendering|Debug|DrawDebugArrow (LocalVariables|GetConstruct_StartingPoint) (LocalVariables|GetConstruct_LineEnd) 5e+01 "(R=1.000000,G=0.000000,B=0.000000,A=1.000000)" 15.0 2.0)
      (Transformation|SetWorldLocation (Variables|Default|GetForwardAxisText) (LocalVariables|GetConstruct_LineEnd) false false))
    (:NewEnumerator1
      (LocalVariables|SetConstruct_LineEnd (+ (LocalVariables|GetConstruct_StartingPoint) (* (LocalVariables|GetConstruct_SplineDirection) (Math|Float|MakeLiteralFloat 1e+02))))
      (Rendering|Debug|DrawDebugArrow (LocalVariables|GetConstruct_StartingPoint) (LocalVariables|GetConstruct_LineEnd) 5e+01 "(R=1.000000,G=0.000000,B=0.000000,A=1.000000)" 15.0 2.0)
      (Transformation|SetWorldLocation (Variables|Default|GetForwardAxisText) (LocalVariables|GetConstruct_LineEnd) false false)
      (LocalVariables|SetConstruct_LineEnd (+ (LocalVariables|GetConstruct_StartingPoint) (* (Math|Vector|RotateVectorAroundAxis (LocalVariables|GetConstruct_SplineDirection) 9e+01 "0.000000,0.000000,1.000000") (Math|Float|MakeLiteralFloat 1e+02))))
      (Rendering|Debug|DrawDebugArrow (LocalVariables|GetConstruct_StartingPoint) (LocalVariables|GetConstruct_LineEnd) 5e+01 "(R=0.000000,G=1.000000,B=0.000000,A=1.000000)" 15.0 2.0)
      (Transformation|SetWorldLocation (Variables|Default|GetRightAxisText) (LocalVariables|GetConstruct_LineEnd) false false))))